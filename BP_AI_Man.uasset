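; AI-controlled melee enemy character that detects and attacks the player.
; Pawn Sensing sets the SeeingPlayer blackboard key when it sees a pawn tagged Player3, and this Blueprint never clears it.
; AttackPlayer plays an attack montage, guarded against re-entry until it completes.
; A forward sphere trace from AttackTracePoint runs as the montage starts, damaging any pawn it hits.
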(event OnSeePawn(PawnSensing)
  (params (Pawn :type Pawn%20Object%20Reference))
  (if (Actor|ActorHasTag Pawn "Player3")
    (AI|Components|Blackboard|SetValueasBool (AI|GetBlackboard (AI|GetAIController self)) (Utilities|Name|MakeLiteralName "SeeingPlayer") true)))

(event Custom|Attack%20Player
  (bind _attack_trace_point (Variables|Default|GetAttack%20Trace%20Point))
  (bind _returnvalue (Transformation|GetWorldLocation _attack_trace_point))
  (if (not (Variables|Default|Getattacking?))
    (Variables|Default|Setattacking? true)
    (Animation|Montage|PlayMontage (Variables|Character|GetMesh) "/Game/ZombieAnimationPack/Animations/Mannequin_UE5/anim_Attack_D_Montage.anim_Attack_D_Montage"
      (:then
        (bind (_outhit _returnvalue_2) (Collision|SphereTraceForObjects _returnvalue (+ _returnvalue (* (Math|Vector|GetForwardVector (Transformation|GetWorldRotation _attack_trace_point)) 2e+02)) 5e+01 (Utilities|Array|MakeArray "ObjectTypeQuery3") false 0 "None"))
        (if _returnvalue_2
          (Game|Damage|ApplyDamage (.HitActor (Collision|BreakHitResult _outhit)) 1e+01 0 0)))
      (:OnCompleted
        (Variables|Default|Setattacking? false)))))

(event EventBeginPlay)

(event Collision|EventActorBeginOverlap
  (params (OtherActor :type Actor%20Object%20Reference)))

(event EventTick
  (params (DeltaSeconds :type Float%20%28single-precision%29)))

(fn ConstructionScript)