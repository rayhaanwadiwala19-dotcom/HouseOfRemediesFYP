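; Interactable box with a hinged lid that can be locked and opened with a matching key held by the player.
; Interaction toggles the lid through a play/reverse timeline with open and close sounds, or checks keys when locked.
; The check compares only the last Keys3 entry to BoxKeyID, then unlocks and opens after the unlock sound.
; A failed check starts a shake timeline, whose rotation node is unwired.
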(event Custom|OpenCloseBox
  ;[0 0.8012 1 0.5] Open/close Logic
  (CallFunction|Sounds)
  (if (Variables|Default|GetBoxClosed?)
    (Variables|Default|SetBoxClosed? false)
    (bind _alpha (Timeline|Box_TL Play)
      (:Update
        (Transformation|SetRelativeRotation (Variables|Default|GetBoxLid) (Math|Rotator|MakeRotator (Math|Float|Lerp 0.0 -1.2e+02 _alpha) 0.0 0.0) false false)))
    (else
      (Variables|Default|SetBoxClosed? true)
      (Timeline|Box_TL Reverse))))

(event Custom|CheckForKey
  (for _array_element (Variables|/Game/VHS_Project_2/VHS_Project_Main/Blueprints/FirstPerson_BP/BP_FirstPersonCharacter.BP_FirstPersonCharacter_C|GetKeys3 (Variables|Default|GetPlayerRef))
    _)
  (if (Utilities|Enum|Equal(Enum) _array_element (Variables|Default|GetBoxKeyID))
    (CallFunction|UnlockBox)
    (else
      (CallFunction|ShakeBox))))

(event Custom|UnlockBox
  (bind _unlocksound (Variables|Default|GetUnlockSound))
  ;[0.15 0.01477 0 0.5] UnlockBox
  (Variables|Default|SetLocked? false)
  (Audio|PlaySoundatLocation _unlocksound (Transformation|GetWorldLocation (Variables|Default|GetBox)) "0, 0, 0" 1.0 1.0 0.0 0 0 0 0)
  (Utilities|FlowControl|Delay (Variables|/Script/Engine.SoundBase|GetDuration _unlocksound))
  (CallFunction|OpenCloseBox))

(event Custom|ShakeBox
  (bind _alpha (Timeline|ShakeDoor_TL PlayFromStart)))

(event EventBeginPlay
  (bind _asbp_first_person_character (Utilities|Casting|CastToBP_FirstPersonCharacter (Game|GetPlayerCharacter 0)))
  (Variables|Default|SetPlayerRef _asbp_first_person_character))

(event EventInteraction
  ;[0 0 1 0.5] Interaction
  (if (Variables|Default|GetLocked?)
    (CallFunction|CheckforKey)
    (else
      (CallFunction|OpenCloseBox))))

(fn ConstructionScript)

(fn Sounds
  (bind _box (Variables|Default|GetBox))
  (bind _returnvalue (Transformation|GetWorldLocation _box))
  (if (Variables|Default|GetLocked?)
    (Audio|PlaySoundatLocation (Variables|Default|GetLockedSound) _returnvalue "0, 0, 0" 1.0 1.0 0.0 0 0 0 0)
    (elif (Variables|Default|GetBoxClosed?)
      (Audio|PlaySoundatLocation (Variables|Default|GetOpenSound) _returnvalue "0, 0, 0" 1.0 1.0 0.0 0 0 0 0)
      (else
        (Audio|PlaySoundatLocation (Variables|Default|GetClosedSound) _returnvalue "0, 0, 0" 1.0 1.0 0.0 0 0 0 0)))))