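; BP_CombinationLock is an interactable three-dial combination lock with a close-up view.
; BeginPlay spawns three indexed BP_Dial actors and attaches them to sockets on the lock mesh.
; Interaction blends the camera to the lock, freezes the player and enables cursor and input, while Q or Escape restores normal play.
; CheckCode compares each dial's number to LockCombination and returns whether all match, though nothing here calls it.
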(event Custom|ExitView
  (bind _returnvalue (Game|GetPlayerController 0))
  (bind _returnvalue_2 (Game|GetPlayerCharacter 0))
  (Game|Player|SetViewTargetwithBlend _returnvalue _returnvalue_2 0.5 "VTBlend_Linear" 0.0 false)
  (Input|DisableInput _returnvalue)
  (Input|ResetIgnoreLookInput _returnvalue)
  (Variables|/Script/Engine.PlayerController|SetbShowMouseCursor _returnvalue false)
  (Pawn|Components|CharacterMovement|SetMovementMode (Variables|/Script/Engine.Character|GetCharacterMovement _returnvalue_2) "MOVE_Walking" 0))

(event EventBeginPlay
  (for _index (range 0 2)
    (bind _returnvalue (Game|SpawnActorfromClass "/Game/InteractionBlueprint/CombinationLock/BP_Dial.BP_Dial_C" (Math|Transform|MakeTransform "0, 0, 0" "0, 0, 0" "1.000000,1.000000,1.000000") "Undefined" "MultiplyWithRoot" 0 _index 0))
    (Utilities|Array|Add (Variables|Default|GetDials) _returnvalue)
    (Transformation|AttachComponentToComponent _returnvalue (Variables|Default|GetSM_CombinationLock) (Utilities|Select :Index _index :Option%200 "Dial01" :Option%201 "Dial02" :Option%202 "Dial03") "KeepRelative" "KeepRelative" "KeepRelative" true)))

(event EventInteraction
  (bind _returnvalue (Game|GetPlayerController 0))
  (Game|Player|SetViewTargetwithBlend (Game|GetPlayerController 0) self 0.5 "VTBlend_Linear" 0.0 false)
  (Pawn|Components|CharacterMovement|DisableMovement (Variables|/Script/Engine.Character|GetCharacterMovement (Game|GetPlayerCharacter 0)))
  (Input|SetIgnoreLookInput _returnvalue true)
  (Utilities|FlowControl|Delay 0.5)
  (Input|EnableInput _returnvalue)
  (Variables|/Script/Engine.PlayerController|SetbShowMouseCursor _returnvalue true))

(event Input|KeyboardEvents|Q
  (params (Key :type Key%20Structure :default "None"))
  (:Pressed
    (CallFunction|ExitView)))

(event Input|KeyboardEvents|Escape
  (params (Key :type Key%20Structure :default "None"))
  (:Pressed
    (CallFunction|ExitView)))

(fn ConstructionScript)

(fn CheckCode
  (bind (_array_element _array_index) (Utilities|Array|ForEachLoopwithBreak (Variables|Default|GetDials) :!label _label)
    (:LoopBody
      (if (== (Variables|/Game/InteractionBlueprint/CombinationLock/BP_Dial.BP_Dial_C|GetNumber _array_element) (Utilities|Array|Get(acopy) (Variables|Default|GetLockCombination) _array_index))
        (LocalVariables|SetLocalSuccess true)
        (else
          (LocalVariables|SetLocalSuccess false)
          (goto _label Break))))
    (:Completed
      (return (LocalVariables|GetLocalSuccess)))))