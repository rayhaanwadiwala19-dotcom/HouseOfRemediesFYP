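; Interactive hinged door for a first-person character, with key lock, optional auto-close and proximity icons.
; Interaction plays timelines for door and handle, using a dot product to swing away from or toward either side based on player position.
; When locked, it compares only the last element of the player's Keys2 to DoorKeyID, then unlocks or shakes.
; A looping timer closes it once the player is far enough; overlap spheres toggle icons.
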(event OnComponentBeginOverlap(InnerIconRadius)
  (params (OverlappedComponent :type Primitive%20Component%20Object%20Reference) (OtherActor :type Actor%20Object%20Reference) (OtherComp :type Primitive%20Component%20Object%20Reference) (OtherBodyIndex :type Integer) (bFromSweep :type Boolean) (SweepResult :type Hit%20Result%20Structure%20%28by%20ref%29))
  (if (== OtherActor (Game|GetPlayerCharacter 0))
    (Development|SetHiddeninGame (Variables|Default|GetInnerIcon) false false)
    (Development|SetHiddeninGame (Variables|Default|GetOuterIcon) true false)))

(event OnComponentEndOverlap(InnerIconRadius)
  (params (OverlappedComponent :type Primitive%20Component%20Object%20Reference) (OtherActor :type Actor%20Object%20Reference) (OtherComp :type Primitive%20Component%20Object%20Reference) (OtherBodyIndex :type Integer))
  (if (== (Game|GetPlayerCharacter 0) OtherActor)
    (Development|SetHiddeninGame (Variables|Default|GetInnerIcon) true false)
    (Development|SetHiddeninGame (Variables|Default|GetOuterIcon) false false)))

(event OnComponentBeginOverlap(OuterIconRadius)
  (params (OverlappedComponent :type Primitive%20Component%20Object%20Reference) (OtherActor :type Actor%20Object%20Reference) (OtherComp :type Primitive%20Component%20Object%20Reference) (OtherBodyIndex :type Integer) (bFromSweep :type Boolean) (SweepResult :type Hit%20Result%20Structure%20%28by%20ref%29))
  (if (== OtherActor (Game|GetPlayerCharacter 0))
    (Development|SetHiddeninGame (Variables|Default|GetOuterIcon) false false)))

(event OnComponentEndOverlap(OuterIconRadius)
  (params (OverlappedComponent :type Primitive%20Component%20Object%20Reference) (OtherActor :type Actor%20Object%20Reference) (OtherComp :type Primitive%20Component%20Object%20Reference) (OtherBodyIndex :type Integer))
  (if (== (Game|GetPlayerCharacter 0) OtherActor)
    (Development|SetHiddeninGame (Variables|Default|GetOuterIcon) true false)))

(event Custom|OpenCloseDoor
  (bind _self self)
  ;[0 1 0.07975 0.5] Open/Close Logic
  (CallFunction|Sounds)
  (if (Variables|Default|GetDoorClosed?)
    (Variables|Default|SetDoorClosed? false)
    (CallFunction|RotateDoorHandle)
    (Variables|Default|SetDotProduct (Math|Vector|DotProduct (Math|Vector|Normalize (- (Transformation|GetActorLocation _self) (Transformation|GetActorLocation (Variables|Default|GetPlayerRef)))) (Transformation|GetActorRightVector _self)))
    (bind _alpha (Timeline|Door_TL Play)
      (:Update
        (Transformation|SetRelativeRotation (Variables|Default|GetDoor) (Math|Rotator|MakeRotator 0.0 0.0 (Math|Float|Lerp 0.0 (Math|Float|SelectFloat 85.0 -85.0 (>= (Variables|Default|GetDotProduct) 0.0)) _alpha)) false false)))
    (else
      (Variables|Default|SetDoorClosed? true)
      (Timeline|Door_TL Reverse))))

(event Custom|AutoClose
  ;[1 0 0.5973 0.5] Auto Close Door
  (if (Variables|Default|GetAutoClose?)
    (Utilities|Time|SetTimerbyEvent (delegate Custom|DoorAutoClose) 2.0 true)))

(event Custom|DoorAutoClose
  ;[1 0 0.5973 0.5] Auto Close Door
  (if (not (Variables|Default|GetDoorClosed?))
    (if (> (Math|Vector|Distance(Vector) (Transformation|GetActorLocation (Variables|Default|GetPlayerRef)) (Transformation|GetActorLocation)) (Variables|Default|GetClosedDistance))
      (CallFunction|OpenCloseDoor))))

(event Custom|CheckForKey
  ;[1 0.7532 0.000492 0.5] KeyCheck
  (for _array_element (Variables|/Game/VHS_Project_2/VHS_Project_Main/Blueprints/FirstPerson_BP/BP_FirstPersonCharacter.BP_FirstPersonCharacter_C|GetKeys2 (Variables|Default|GetPlayerRef))
    _)
  (if (Utilities|Enum|Equal(Enum) _array_element (Variables|Default|GetDoorKeyID))
    (CallFunction|UnlockDoor)
    (else
      (CallFunction|ShakeDoor))))

(event Custom|RotateDoorHandle
  ;[0.1419 0 1 0.5] Door Handle Rotation
  (bind _newtrack_1 (Timeline|DoorHandle_TL PlayFromStart)
    (:Update
      (Transformation|SetRelativeRotation (Variables|Default|GetDoorHandle) (Math|Rotator|MakeRotator 0.0 _newtrack_1 0.0) false false))))

(event Custom|UnlockDoor
  (bind _unlocksound (Variables|Default|GetUnlockSound))
  ;[0.15 0.15 0.15 0.5] UnlockDoor
  (Variables|Default|SetLocked? false)
  (Audio|PlaySoundatLocation _unlocksound (Transformation|GetWorldLocation (Variables|Default|GetDoor)) "0, 0, 0" 1.0 1.0 0.0 0 0 0 0)
  (Utilities|FlowControl|Delay (Variables|/Script/Engine.SoundBase|GetDuration _unlocksound))
  (CallFunction|OpenCloseDoor))

(event Custom|ShakeDoor
  ;[0.04924 1 0.2778 0.5] Comment
  (CallFunction|RotateDoorHandle)
  (bind _newtrack_1 (Timeline|ShakeDoor_TL PlayFromStart)
    (:Update
      (Transformation|SetRelativeRotation (Variables|Default|GetDoor) (Math|Rotator|MakeRotator 0.0 0.0 _newtrack_1) false false))))

(event EventBeginPlay
  (bind _asbp_first_person_character (Utilities|Casting|CastToBP_FirstPersonCharacter (Game|GetPlayerCharacter 0)))
  (Variables|Default|SetPlayerRef _asbp_first_person_character)
  (CallFunction|AutoClose))

(event EventInteraction
  ;[0 0.8008 1 0.5] Interaction
  (if (Variables|Default|GetLocked?)
    (CallFunction|CheckforKey)
    (else
      (CallFunction|OpenCloseDoor))))

(fn ConstructionScript
  (Utilities|FlowControl|Sequence
    (:then_1
      (Transformation|SetWorldScale3D (Variables|Default|GetOuterIcon) (Math|Conversions|ToVector(Float) (/ (Variables|Default|GetIconSize) 1e+01)))
      (Transformation|SetRelativeLocation (Variables|Default|GetOuterIcon) (Variables|Default|GetIcon%20Location) false false))
    (:then_2
      (Components|Sphere|SetSphereRadius (Variables|Default|GetInnerIconRadius) (Variables|Default|GetInnerRadius) true)
      (Components|Sphere|SetSphereRadius (Variables|Default|GetOuterIconRadius) (Variables|Default|GetOuterRadius) true))))

(fn Sounds
  (bind _door (Variables|Default|GetDoor))
  (bind _returnvalue (Transformation|GetWorldLocation _door))
  (if (Variables|Default|GetLocked?)
    (Audio|PlaySoundatLocation (Variables|Default|GetLockedSound) _returnvalue "0, 0, 0" 1.0 1.0 0.0 0 0 0 0)
    (elif (Variables|Default|GetDoorClosed?)
      (Audio|PlaySoundatLocation (Variables|Default|GetOpenSound) _returnvalue "0, 0, 0" 1.0 1.0 0.0 0 0 0 0)
      (else
        (Audio|PlaySoundatLocation (Variables|Default|GetCloseSound) _returnvalue "0, 0, 0" 1.0 1.0 0.0 0 0 0 0)))))