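; BP_Dresser01 is an interactive dresser whose drawers slide open and closed.
; Its Interaction event ignores the SMDresser01 body by name and passes any other component to OpenDrawer.
; OpenDrawer checks the component's relative Y, then plays or reverses one shared timeline that lerps that position, with a 2D drawer sound either way.
; A DrawerOpening flag blocks new requests until the timeline finishes.
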(event Custom|OpenDrawer
  (params (Component :type Primitive%20Component%20Object%20Reference))
  (bind _relativelocation (Variables|/Script/Engine.SceneComponent|GetRelativeLocation Component))
  (if (not (Variables|Default|GetDrawerOpening))
    (Variables|Default|SetDrawerOpening true)
    (if (not (> (.y _relativelocation) 29.0))
      (Audio|PlaySound2D "/Game/DresserBluePrint/Audio/152529__dwoboyle__drawer-wooden-junk-open-01.152529__dwoboyle__drawer-wooden-junk-open-01" 1.0 1.0 0.0 0 0)
      (bind _alpha (Timeline|OpenDrawer_TL PlayFromStart)
        (:Update
          (Transformation|SetRelativeLocation Component (Math|Vector|MakeVector (.x _relativelocation) (Math|Float|Lerp 3.0 3e+01 _alpha) (.z _relativelocation)) false false))
        (:Finished
          (Variables|Default|SetDrawerOpening false)))
      (else
        (Audio|PlaySound2D "/Game/DresserBluePrint/Audio/152529__dwoboyle__drawer-wooden-junk-open-01.152529__dwoboyle__drawer-wooden-junk-open-01" 1.0 1.0 0.0 0 0)
        (Timeline|OpenDrawer_TL ReverseFromEnd)))))

(event EventBeginPlay)

(event EventInteraction
  (params (Component :type Primitive%20Component%20Object%20Reference))
  (if (not (Utilities|Enum|Equal(Enum) (Utilities|GetObjectName Component) (Utilities|GetObjectName (Variables|Default|GetSM_Dresser01))))
    (CallFunction|OpenDrawer Component)))

(fn ConstructionScript)