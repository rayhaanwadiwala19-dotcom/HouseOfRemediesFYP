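; BP_FuelCan is a fuel can pickup that feeds the state of the generator puzzle.
; On BeginPlay it caches the BP_GeneratorPuzzle actor through GetActorOfClass.
; On Interaction it sets that puzzle's HasFuelCan flag and destroys itself, or plays a 2D "hands are full" cue if the flag is already set.
; The carried state lives on the puzzle actor, so only one can is held at a time.
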(event EventBeginPlay
  (bind _returnvalue (Actor|GetActorOfClass "/Game/InteractionBlueprint/GeneratorPuzzle/BP_GeneratorPuzzle.BP_GeneratorPuzzle_C"))
  (Variables|Default|SetGeneratorPuzzleRef _returnvalue))

(event EventInteraction
  (if (Variables|/Game/InteractionBlueprint/GeneratorPuzzle/BP_GeneratorPuzzle.BP_GeneratorPuzzle_C|GetHasFuelCan (Variables|Default|GetGeneratorPuzzleRef))
    (Audio|PlaySound2D "/Game/InteractionBlueprint/GeneratorPuzzle/Audio/MyHandsAreFull_Cue.MyHandsAreFull_Cue" 1.0 1.0 0.0 0 0)
    (else
      (Variables|/Game/InteractionBlueprint/GeneratorPuzzle/BP_GeneratorPuzzle.BP_GeneratorPuzzle_C|SetHasFuelCan (Variables|Default|GetGeneratorPuzzleRef) true)
      (Actor|DestroyActor))))

(fn ConstructionScript
  (|CallParentFunction))