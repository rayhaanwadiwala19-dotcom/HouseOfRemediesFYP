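; Generator puzzle actor that the player refuels with fuel cans in two pours to switch it on.
; A box overlap shows and removes the generator widget for the player.
; Interaction with a can plays pour audio and a can-tilt timeline, while separate first and second pour timelines raise the fuel level to half, then full.
; At full fuel it fades in the running loop and calls the puzzle-finish dispatcher.
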(event OnComponentBeginOverlap(Box)
  (params (OverlappedComponent :type Primitive%20Component%20Object%20Reference) (OtherActor :type Actor%20Object%20Reference) (OtherComp :type Primitive%20Component%20Object%20Reference) (OtherBodyIndex :type Integer) (bFromSweep :type Boolean) (SweepResult :type Hit%20Result%20Structure%20%28by%20ref%29))
  ;[0.15 0.15 0.15 0.5] DisplayingWidget
  (if (== OtherActor (Game|GetPlayerCharacter 0))
    (bind _returnvalue (UserInterface|CreateWidget "/Game/InteractionBlueprint/GeneratorPuzzle/Widgets/W_Generator.W_Generator_C"))
    (bind _output_get (Variables|Default|SetGeneratorWidgetRef _returnvalue))
    (UserInterface|Viewport|AddtoViewport _output_get 0)))

(event OnComponentEndOverlap(Box)
  (params (OverlappedComponent :type Primitive%20Component%20Object%20Reference) (OtherActor :type Actor%20Object%20Reference) (OtherComp :type Primitive%20Component%20Object%20Reference) (OtherBodyIndex :type Integer))
  ;[0.15 0.15 0.15 0.5] DisplayingWidget
  (if (== (Game|GetPlayerCharacter 0) OtherActor)
    (Widget|RemovefromParent (Variables|Default|GetGeneratorWidgetRef))))

(event Custom|FillGenerator
  (bind _generatoronloop_cue (Variables|Default|GetGeneratorOnLoop_Cue))
  (Audio|PlaySoundatLocation "/Game/InteractionBlueprint/GeneratorPuzzle/Audio/LiquidPouring_Cue.LiquidPouring_Cue" (Transformation|GetWorldLocation (Variables|Default|GetGenerator)) "0, 0, 0" 1.0 1.0 0.0 0 0 0 0)
  (CallFunction|FuelCanAnim)
  (if (not (Variables|Default|GetFilledOnce))
    (bind _alpha (Timeline|FuelPouringFirstTime Play)
      (:Update
        (Variables|Default|SetFuelLevel (Math|Float|Lerp 0.0 5e+01 _alpha))
        (if (< (Variables|Default|GetFuelLevel) 1e+02) :!label _label
          (Variables|Default|SetHasFuelCan false)
          (else
            (bind _output_get (Variables|Default|SetGeneratorOn (>= (Variables|Default|GetFuelLevel) 1e+02)))
            (if _output_get
              (Audio|Components|Audio|FadeIn _generatoronloop_cue 1.0 1.0 0.0 "Linear" :!class /Script/Engine.AudioComponent)
              (Audio|Components|Audio|SetVolumeMultiplier _generatoronloop_cue 1.0 :!class /Script/Engine.AudioComponent)
              (Default|CallEVDGeneratorPuzzleFinish)))))
      (:Finished
        (Variables|Default|SetFilledOnce true)))
    (else
      (bind _alpha_2 (Timeline|FuelPouringSecondTime Play)
        (:Update
          (Variables|Default|SetFuelLevel (Math|Float|Lerp 51.0 1e+02 _alpha_2))
          (goto _label))))))

(event Custom|FuelCanAnim
  (bind _fuelcan (Variables|Default|GetFuelCan))
  (bind _relativerotation (Variables|/Script/Engine.SceneComponent|GetRelativeRotation _fuelcan))
  ;[0.15 0.15 0.15 0.5] FuelcanPouringAnim
  (Rendering|SetVisibility (Variables|Default|GetFuelCan) true false)
  (bind _alpha (Timeline|FuelCanAnim_TL PlayFromStart)
    (:Update
      (Transformation|SetRelativeRotation _fuelcan (Math|Rotator|MakeRotator (.roll _relativerotation) (Math|Float|Lerp 35.0 85.0 _alpha) (.yaw _relativerotation)) false false)
      (Utilities|FlowControl|Delay 3.0)
      (Rendering|SetVisibility (Variables|Default|GetFuelCan) false false))
    (:Finished
      (Utilities|FlowControl|Delay 1.0)
      (Timeline|FuelCanAnim_TL Reverse))))

(event EventBeginPlay)

(event Collision|EventActorBeginOverlap
  (params (OtherActor :type Actor%20Object%20Reference)))

(event EventTick
  (params (DeltaSeconds :type Float%20%28single-precision%29)))

(event EventInteraction
  ;[0.15 0.15 0.15 0.5] Interaction
  (if (Variables|Default|GetHasFuelCan)
    (CallFunction|FillGenerator)))

(fn ConstructionScript)