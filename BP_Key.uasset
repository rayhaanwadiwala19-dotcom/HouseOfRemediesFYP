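; BP_Key is a key pickup that gives its KeyID to the first-person player character.
; On Interaction it calls AddKeys on the player reference cached at BeginPlay, destroys itself and plays a 2D pickup sound.
; Two overlap spheres toggle proximity icons, showing the outer icon at range and swapping to the inner icon up close.
; The construction script applies the configurable mesh, icon size and location, and both sphere radii.
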(event OnComponentBeginOverlap(InnerIconRadius)
  (params (OverlappedComponent :type Primitive%20Component%20Object%20Reference) (OtherActor :type Actor%20Object%20Reference) (OtherComp :type Primitive%20Component%20Object%20Reference) (OtherBodyIndex :type Integer) (bFromSweep :type Boolean) (SweepResult :type Hit%20Result%20Structure%20%28by%20ref%29))
  ;[0.15 0.15 0.15 0.5] Inner&OuterIcons
  (if (== OtherActor (Game|GetPlayerCharacter 0))
    (Development|SetHiddeninGame (Variables|Default|GetInnerIcon) false false)
    (Development|SetHiddeninGame (Variables|Default|GetOuterIcon) true false)))

(event OnComponentEndOverlap(InnerIconRadius)
  (params (OverlappedComponent :type Primitive%20Component%20Object%20Reference) (OtherActor :type Actor%20Object%20Reference) (OtherComp :type Primitive%20Component%20Object%20Reference) (OtherBodyIndex :type Integer))
  ;[0.15 0.15 0.15 0.5] Inner&OuterIcons
  (if (== (Game|GetPlayerCharacter 0) OtherActor)
    (Development|SetHiddeninGame (Variables|Default|GetInnerIcon) true false)
    (Development|SetHiddeninGame (Variables|Default|GetOuterIcon) false false)))

(event OnComponentBeginOverlap(OuterIconRadius)
  (params (OverlappedComponent :type Primitive%20Component%20Object%20Reference) (OtherActor :type Actor%20Object%20Reference) (OtherComp :type Primitive%20Component%20Object%20Reference) (OtherBodyIndex :type Integer) (bFromSweep :type Boolean) (SweepResult :type Hit%20Result%20Structure%20%28by%20ref%29))
  ;[0.15 0.15 0.15 0.5] Inner&OuterIcons
  (if (== OtherActor (Game|GetPlayerCharacter 0))
    (Development|SetHiddeninGame (Variables|Default|GetOuterIcon) false false)))

(event OnComponentEndOverlap(OuterIconRadius)
  (params (OverlappedComponent :type Primitive%20Component%20Object%20Reference) (OtherActor :type Actor%20Object%20Reference) (OtherComp :type Primitive%20Component%20Object%20Reference) (OtherBodyIndex :type Integer))
  ;[0.15 0.15 0.15 0.5] Inner&OuterIcons
  (if (== (Game|GetPlayerCharacter 0) OtherActor)
    (Development|SetHiddeninGame (Variables|Default|GetOuterIcon) true false)))

(event EventBeginPlay
  (bind _asbp_first_person_character (Utilities|Casting|CastToBP_FirstPersonCharacter (Game|GetPlayerCharacter 0)))
  (Variables|Default|SetPlayerRef _asbp_first_person_character))

(event EventInteraction
  (params (Component :type Primitive%20Component%20Object%20Reference))
  (Default|AddKeys (Variables|Default|GetPlayerRef) (Variables|Default|GetKeyID))
  (Actor|DestroyActor)
  (Audio|PlaySound2D "/Game/InteractionBlueprint/Door/Audio/KeyPicked.KeyPicked" 1.0 1.0 0.0 0 0))

(fn ConstructionScript
  (Utilities|FlowControl|Sequence
    (:then_0
      (Components|StaticMesh|SetStaticMesh (Variables|Default|GetStaticMesh) (Variables|Default|GetKeyMesh)))
    (:then_1
      (Transformation|SetWorldScale3D (Variables|Default|GetOuterIcon) (Math|Conversions|ToVector(Float) (/ (Variables|Default|GetIconSize) 1e+01)))
      (Transformation|SetRelativeLocation (Variables|Default|GetOuterIcon) (Variables|Default|GetIconLocation) false false))
    (:then_2
      (Components|Sphere|SetSphereRadius (Variables|Default|GetInnerIconRadius) (Variables|Default|GetInnerRadius) true)
      (Components|Sphere|SetSphereRadius (Variables|Default|GetOuterIconRadius) (Variables|Default|GetOutterRadius) true))))