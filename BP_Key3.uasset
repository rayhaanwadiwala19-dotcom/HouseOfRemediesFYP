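; BP_Key3 is a pickup key actor that gives the player a key when interacted with.
; On BeginPlay it caches the player as BP_FirstPersonCharacter, and on Interaction it passes its KeyID to the character's AddKeys3 and destroys itself.
; The construction script applies the configurable KeyMesh to the StaticMesh component.
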(event EventBeginPlay
  (bind _asbp_first_person_character (Utilities|Casting|CastToBP_FirstPersonCharacter (Game|GetPlayerCharacter 0)))
  (Variables|Default|SetPlayerRef _asbp_first_person_character))

(event EventInteraction
  (Default|AddKeys3 (Variables|Default|GetPlayerRef) (Variables|Default|GetKeyID))
  (Actor|DestroyActor))

(fn ConstructionScript
  (Components|StaticMesh|SetStaticMesh (Variables|Default|GetStaticMesh) (Variables|Default|GetKeyMesh)))