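; Interactive lights-out style keypad puzzle with ten buttons, completed when every button is lit.
; Interaction blends the camera to the keypad, freezes the player and shows the cursor; Q exits and restores control.
; Mouse clicks line trace to a button mesh, toggling its state and material plus any linked buttons from ButtonConfig.
; When all states are on, it fires the KeyPadCompleted dispatcher and exits the view.
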(event Custom|ExitView
  (bind _returnvalue (Game|GetPlayerController 0))
  (bind _returnvalue_2 (Game|GetPlayerCharacter 0))
  (Game|Player|SetViewTargetwithBlend _returnvalue _returnvalue_2 0.5 "VTBlend_Linear" 0.0 false)
  (Input|DisableInput _returnvalue)
  (Input|ResetIgnoreLookInput _returnvalue)
  (Pawn|Components|CharacterMovement|SetMovementMode (Variables|/Script/Engine.Character|GetCharacterMovement _returnvalue_2) "MOVE_Walking" 0)
  (Variables|/Script/Engine.PlayerController|SetbShowMouseCursor _returnvalue false))

(event EventInteraction
  (params (Component :type Primitive%20Component%20Object%20Reference))
  (bind _returnvalue (Game|GetPlayerController 0))
  (Game|Player|SetViewTargetwithBlend (Game|GetPlayerController 0) self 0.5 "VTBlend_Linear" 0.0 false)
  (Pawn|Components|CharacterMovement|DisableMovement (Variables|/Script/Engine.Character|GetCharacterMovement (Game|GetPlayerCharacter 0)))
  (Input|SetIgnoreLookInput _returnvalue true)
  (Utilities|FlowControl|Delay 0.5)
  (Input|EnableInput _returnvalue)
  (Variables|/Script/Engine.PlayerController|SetbShowMouseCursor _returnvalue true))

(event Input|KeyboardEvents|Q
  (params (Key :type Key%20Structure :default "None"))
  (:Pressed
    (CallFunction|ExitView)))

(event Input|MouseEvents|LeftMouseButton
  (params (Key :type Key%20Structure :default "None"))
  (bind _returnvalue (Game|GetPlayerController 0))
  (bind (_worldlocation _worlddirection _returnvalue_2) (Game|Player|ConvertMouseLocationToWorldSpace _returnvalue))
  (:Pressed
    (Utilities|IsValid _returnvalue
      (:Is%20Valid
        (if _returnvalue_2
          (bind (_outhit _returnvalue_3) (Collision|LineTraceByChannel _worldlocation (+ _worldlocation (* _worlddirection 1.5e+02)) "TraceTypeQuery1" false 0 "None" false))
          (if _returnvalue_3
            (Audio|PlaySound2D "/Game/InteractionBlueprint/KeyPad/ButtonPress.ButtonPress" 1.0 1.0 0.0 0 0)
            (Development|PrintString (Utilities|GetObjectName (.HitComponent (Collision|BreakHitResult _outhit))))
            (bind _asstatic_mesh_component (Utilities|Casting|CastToStaticMeshComponent (.HitComponent (Collision|BreakHitResult _outhit))))
            (CallFunction|ToggleActivation (Utilities|Array|FindItem (Variables|Default|GetButtons) _asstatic_mesh_component))
            (if (.ReturnValue (Utilities|Map|Find (Variables|Default|GetButtonConfig) (Utilities|Array|FindItem (Variables|Default|GetButtons) _asstatic_mesh_component)))
              (for _array_element (Utilities|Struct|BreakS_ButtonsToActivate (.Value (Utilities|Map|Find (Variables|Default|GetButtonConfig) (Utilities|Array|FindItem (Variables|Default|GetButtons) _asstatic_mesh_component))))
                (CallFunction|ToggleActivation _array_element)))
            (bind _success (CallFunction|CheckAnswer))
            (if _success
              (Utilities|FlowControl|Delay 0.5)
              (Default|CallEVDKeyPadCompleted)
              (CallFunction|ExitView))))))))

(fn ConstructionScript
  (Variables|Default|SetButtons (Utilities|Array|MakeArray (Variables|Default|GetSM_Button0) (Variables|Default|GetSM_Button1) (Variables|Default|GetSM_Button2) (Variables|Default|GetSM_Button3) (Variables|Default|GetSM_Button4) (Variables|Default|GetSM_Button5) (Variables|Default|GetSM_Button6) (Variables|Default|GetSM_Button7) (Variables|Default|GetSM_Button8) (Variables|Default|GetSM_Button9))))

(fn ToggleActivation
  (params (Buttonindex :type Integer))
  (bind _buttonactivationstate (Variables|Default|GetButtonActivationState))
  (bind _buttons (Variables|Default|GetButtons))
  (bind _output (Utilities|Array|Get(acopy) _buttons Buttonindex))
  (Utilities|Array|SetArrayElem _buttonactivationstate Buttonindex (not (Utilities|Array|Get(acopy) _buttonactivationstate Buttonindex)))
  (if (Utilities|Array|Get(acopy) _buttonactivationstate Buttonindex)
    (Rendering|Material|SetMaterial _output 0 "/Game/InteractionBlueprint/KeyPad/M_ButtonOn.M_ButtonOn")
    (else
      (Rendering|Material|SetMaterial _output 0 "/Game/InteractionBlueprint/KeyPad/M_ButtonOff.M_ButtonOff"))))

(fn CheckAnswer
  (if (== (Utilities|Array|Length (Variables|Default|GetButtons)) (Utilities|Array|Length (Variables|Default|GetButtonActivationState)))
    (for _array_element (Variables|Default|GetButtonActivationState)
      (if (not _array_element)
        (return false)))
    (return true)))