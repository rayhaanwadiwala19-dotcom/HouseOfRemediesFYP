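; BP_Pills is a pickup actor that gives the first-person character pills when V is pressed nearby.
; A sphere overlap with BP_FirstPersonCharacter enables player 0's input on the actor, and leaving disables it.
; The V press uses the overlap's OtherActor to set HasPills and show the character's Pills component.
; It also destroys its own Pills component, not the whole actor, and plays a 2D sound.
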(event OnComponentBeginOverlap(Sphere)
  (params (OverlappedComponent :type Primitive%20Component%20Object%20Reference) (OtherActor :type Actor%20Object%20Reference) (OtherComp :type Primitive%20Component%20Object%20Reference) (OtherBodyIndex :type Integer) (bFromSweep :type Boolean) (SweepResult :type Hit%20Result%20Structure%20%28by%20ref%29))
  (Utilities|Casting|CastToBP_FirstPersonCharacter OtherActor)
  (Input|EnableInput (Game|GetPlayerController 0)))

(event OnComponentEndOverlap(Sphere)
  (params (OverlappedComponent :type Primitive%20Component%20Object%20Reference) (OtherActor :type Actor%20Object%20Reference) (OtherComp :type Primitive%20Component%20Object%20Reference) (OtherBodyIndex :type Integer))
  (Utilities|Casting|CastToBP_FirstPersonCharacter OtherActor)
  (Input|DisableInput (Game|GetPlayerController 0)))

(event EventBeginPlay)

(event Collision|EventActorBeginOverlap
  (params (OtherActor :type Actor%20Object%20Reference)))

(event EventTick
  (params (DeltaSeconds :type Float%20%28single-precision%29)))

(event Input|KeyboardEvents|V
  (params (Key :type Key%20Structure :default "None"))
  (:Pressed
    (bind _asbp_first_person_character (Utilities|Casting|CastToBP_FirstPersonCharacter (stale OnComponentBeginOverlap(Sphere) OtherActor)))
    (Variables|/Game/VHS_Project_2/VHS_Project_Main/Blueprints/FirstPerson_BP/BP_FirstPersonCharacter.BP_FirstPersonCharacter_C|SetHasPills? _asbp_first_person_character true)
    (Components|DestroyComponent (Variables|Default|GetPills))
    (Audio|PlaySound2D "/Game/SanitySystem/Audio/Pills.Pills" 1.0 1.0 0.0 0 0)
    (Rendering|SetVisibility (Variables|/Game/VHS_Project_2/VHS_Project_Main/Blueprints/FirstPerson_BP/BP_FirstPersonCharacter.BP_FirstPersonCharacter_C|Getpills _asbp_first_person_character) true false)))

(fn ConstructionScript)