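; Trigger volume actor that prepares a referenced Jumpscare actor when the player enters it.
; While Active, the main Box calls PrepareJumpscare once, then destroys the trigger unless UseToggleActorActive is set.
; With that flag, separate Enable and Disable volumes switch the jumpscare's active state on player overlap; without it, the construction script removes them and their text labels.
; BeginPlay limits the Box to pawn overlaps.
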(event OnComponentBeginOverlap(Box)
  (params (OverlappedComponent :type Primitive%20Component%20Object%20Reference) (OtherActor :type Actor%20Object%20Reference) (OtherComp :type Primitive%20Component%20Object%20Reference) (OtherBodyIndex :type Integer) (bFromSweep :type Boolean) (SweepResult :type Hit%20Result%20Structure%20%28by%20ref%29))
  ;[0 0 0] Trigger Jumpscare
  (Utilities|IsPlayer OtherActor)
  (if (Variables|Settings|GetActive)
    (Utilities|FlowControl|DoOnce false
      (:Completed
        (bind _jumpscare (Variables|Settings|GetJumpscare)
          (:then
            (Default|PrepareJumpscare _jumpscare)
            (if (not (Variables|Settings|Optimization|GetUseToggleActorActive))
              (Actor|DestroyActor)))
          (:else))))))

(event OnComponentBeginOverlap(Enable)
  (params (OverlappedComponent :type Primitive%20Component%20Object%20Reference) (OtherActor :type Actor%20Object%20Reference) (OtherComp :type Primitive%20Component%20Object%20Reference) (OtherBodyIndex :type Integer) (bFromSweep :type Boolean) (SweepResult :type Hit%20Result%20Structure%20%28by%20ref%29))
  ;[0 0 0] Toggle Actor
  (Utilities|IsPlayer OtherActor)
  (bind _jumpscare (Variables|Settings|GetJumpscare)
    (:then
      (Default|ToggleActorActive _jumpscare true))
    (:else)))

(event OnComponentBeginOverlap(Disable)
  (params (OverlappedComponent :type Primitive%20Component%20Object%20Reference) (OtherActor :type Actor%20Object%20Reference) (OtherComp :type Primitive%20Component%20Object%20Reference) (OtherBodyIndex :type Integer) (bFromSweep :type Boolean) (SweepResult :type Hit%20Result%20Structure%20%28by%20ref%29))
  ;[0 0 0] Toggle Actor
  (Utilities|IsPlayer OtherActor)
  (bind _jumpscare (Variables|Settings|GetJumpscare)
    (:then
      (Default|ToggleActorActive _jumpscare false))
    (:else)))

(event EventBeginPlay
  ;[0 0 0] Begin Play
  (CallFunction|SetCollision))

(fn ConstructionScript
  (if (not (Variables|Settings|Optimization|GetUseToggleActorActive))
    (Components|DestroyComponent (Variables|Default|GetEnable))))

(fn SetCollision
  (bind _box (Variables|Default|GetBox))
  ;[0 0 0] Set Collision
  (Collision|SetCollisionEnabled _box "QueryOnly")
  (Collision|SetCollisionResponsetoAllChannels _box "ECR_Ignore")
  (Collision|SetCollisionResponsetoChannel _box "ECC_Pawn" "ECR_Overlap")
  (return))