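; Rotating table puzzle piece that the player turns in quarter steps until every table in the level sits at its answer position.
; Interaction sets Finalized by comparing the next position to PuzzleAnswer, then a timeline rotates the table with a slide sound.
; Each instance polls all tables on a looping timer and calls the completion event once all are finalized.
; Overlap spheres swap proximity icons, sized in construction, and Tick prints debug state.
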(event OnComponentBeginOverlap(InnerIconRadius)
  (params (OverlappedComponent :type Primitive%20Component%20Object%20Reference) (OtherActor :type Actor%20Object%20Reference) (OtherComp :type Primitive%20Component%20Object%20Reference) (OtherBodyIndex :type Integer) (bFromSweep :type Boolean) (SweepResult :type Hit%20Result%20Structure%20%28by%20ref%29))
  (if (== OtherActor (Game|GetPlayerCharacter 0))
    (Development|SetHiddeninGame (Variables|Default|GetInnerIcon) false false)
    (Development|SetHiddeninGame (Variables|Default|GetOuterIcon) true false)))

(event OnComponentEndOverlap(InnerIconRadius)
  (params (OverlappedComponent :type Primitive%20Component%20Object%20Reference) (OtherActor :type Actor%20Object%20Reference) (OtherComp :type Primitive%20Component%20Object%20Reference) (OtherBodyIndex :type Integer))
  (if (== (Game|GetPlayerCharacter 0) OtherActor)
    (Development|SetHiddeninGame (Variables|Default|GetInnerIcon) true false)
    (Development|SetHiddeninGame (Variables|Default|GetOuterIcon) false false)))

(event OnComponentBeginOverlap(OuterIconRadius)
  (params (OverlappedComponent :type Primitive%20Component%20Object%20Reference) (OtherActor :type Actor%20Object%20Reference) (OtherComp :type Primitive%20Component%20Object%20Reference) (OtherBodyIndex :type Integer) (bFromSweep :type Boolean) (SweepResult :type Hit%20Result%20Structure%20%28by%20ref%29))
  (if (== OtherActor (Game|GetPlayerCharacter 0))
    (Development|SetHiddeninGame (Variables|Default|GetOuterIcon) false false)))

(event OnComponentEndOverlap(OuterIconRadius)
  (params (OverlappedComponent :type Primitive%20Component%20Object%20Reference) (OtherActor :type Actor%20Object%20Reference) (OtherComp :type Primitive%20Component%20Object%20Reference) (OtherBodyIndex :type Integer))
  (if (== (Game|GetPlayerCharacter 0) OtherActor)
    (Development|SetHiddeninGame (Variables|Default|GetOuterIcon) true false)))

(event Custom|RotateTable
  (if (not (Variables|Default|GetTableMoving))
    (Variables|Default|SetTableMoving true)
    (Audio|PlaySound2D "/Game/InteractionBlueprint/LargeStatuePuzzle/Audio/WoodSlide_Cue.WoodSlide_Cue" 1.0 1.0 0.0 0 0)
    (bind _alpha (Timeline|TableRotation PlayFromStart)
      (:Update
        (Transformation|SetRelativeRotation (Variables|Default|GetRotatingTable) (Math|Rotator|MakeRotator 0.0 0.0 (Math|Float|Lerp (.yaw (Variables|Default|GetStartingRotationTable)) (- (.yaw (Variables|Default|GetStartingRotationTable)) 9e+01) _alpha)) false false))
      (:Finished
        (Variables|Default|SetStartingRotationTable (Math|Rotator|MakeRotator 0.0 0.0 (Math|Float|Lerp (.yaw (Variables|Default|GetStartingRotationTable)) (- (.yaw (Variables|Default|GetStartingRotationTable)) 9e+01) _alpha)))
        (Variables|Default|SetTableMoving false)
        (bind _result (Math|Integer|IncrementInt (Variables|Default|GetTablePosition))
          (:%20%20
            (bind _output_get (Variables|Default|SetTablePosition _result))
            (if (> _output_get 3)
              (Variables|Default|SetTablePosition 0))))))))

(event Custom|PuzzleCheck
  (Variables|Default|SetPuzzleSolved true)
  (for _array_element (Variables|Default|GetAllTables)
    (if (not (Variables|BP_Rotating_Master_Puzzle_C|GetFinalized _array_element))
      (Variables|Default|SetPuzzleSolved false)))
  (if (Variables|Default|GetPuzzleSolved)
    (Utilities|Time|ClearandInvalidateTimerbyHandle (stale EventBeginPlay _returnvalue))
    (Default|CallEVDPuzzleCompleted)))

(event EventInteraction
  (params (Component :type Primitive%20Component%20Object%20Reference))
  (if (== (+ (Variables|Default|GetTablePosition) 1) (Variables|Default|GetPuzzleAnswer))
    (Variables|Default|SetFinalized true)
    (CallFunction|RotateTable)
    (else
      (Variables|Default|SetFinalized false)
      (CallFunction|RotateTable))))

(event EventBeginPlay
  (Variables|Default|SetStartingRotationTable (Variables|/Script/Engine.SceneComponent|GetRelativeRotation (Variables|Default|GetRotatingTable)))
  (bind _outactors (Actor|GetAllActorsOfClass "BP_Rotating_Master_Puzzle_C"))
  (Variables|Default|SetAllTables _outactors)
  (bind _returnvalue (Utilities|Time|SetTimerbyEvent (delegate Custom|PuzzleCheck) 0.25 true)))

(event EventTick
  (params (DeltaSeconds :type Float%20%28single-precision%29))
  (Development|PrintString (Utilities|String|ToString(Integer) (Variables|Default|GetTablePosition)) true true "(R=0.000000,G=0.660000,B=1.000000,A=1.000000)" DeltaSeconds)
  (Development|PrintString (Utilities|String|ToString(Boolean) (Variables|Default|GetFinalized)) true true "(R=0.000000,G=0.660000,B=1.000000,A=1.000000)" DeltaSeconds))

(fn ConstructionScript
  (Utilities|FlowControl|Sequence
    (:then_0
      (|CallParentFunction))
    (:then_1
      (Transformation|SetWorldScale3D (Variables|Default|GetOuterIcon) (Math|Conversions|ToVector(Float) (/ (Variables|Default|GetIconSize) 1e+01)))
      (Transformation|SetRelativeLocation (Variables|Default|GetOuterIcon) (Variables|Default|GetIconLocation) false false))
    (:then_2
      (Components|Sphere|SetSphereRadius (Variables|Default|GetInnerIconRadius) (Variables|Default|GetInnerRadius) true)
      (Components|Sphere|SetSphereRadius (Variables|Default|GetOuterIconRadius) (Variables|Default|GetOuterRadius) true))))