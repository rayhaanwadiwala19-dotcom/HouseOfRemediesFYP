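; One-shot box trigger that plays a jumpscare when the player overlaps it while Active, then destroys itself.
; Depending on its settings it runs a ShockLink camera scare, a photo scare with async-loaded sound/image and camera shake, or starts a linked Jumpscare actor.
; Actor scares can wait on timers until recently rendered, with a timeout that fires or skips them.
; Scares chain by activating other listed jumpscares and prepare actors.
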(event OnComponentBeginOverlap(Box)
  (params (OverlappedComponent :type Primitive%20Component%20Object%20Reference) (OtherActor :type Actor%20Object%20Reference) (OtherComp :type Primitive%20Component%20Object%20Reference) (OtherBodyIndex :type Integer) (bFromSweep :type Boolean) (SweepResult :type Hit%20Result%20Structure%20%28by%20ref%29))
  ;[0 0 0] Trigger Jumpscare
  (if (== OtherActor (Game|GetPlayerCharacter 0))
    (if (Variables|Settings|GetActive)
      (Utilities|FlowControl|DoOnce false
        (:Completed
          (CallFunction|SetData)
          (if (Variables|Settings|Jumpscare|ShockLink|GetUseShockLink)
            ;;[0 0 0] Camera Jumpscare
            (Utilities|👻StartShockLink👻 (Variables|Settings|Jumpscare|ShockLink|GetShockLink_Data)
              (:Completed
                (CallFunction|ActivateJumpscares)
                (Actor|DestroyActor)))
            (elif (Variables|Settings|Jumpscare|PhotoScare|GetUsePhotoScare)
              (if (and (Variables|Settings|Jumpscare|Sound|GetUseJumpscareSound) (Variables|Settings|Jumpscare|PhotoScare|GetUsePhotoScare)) :!label _label
                ;;[0 0 0] Widget / Sound
                (if (Utilities|IsValidSoftObjectReference (Variables|Settings|Jumpscare|PhotoScare|GetImage))
                  (if (Variables|Settings|Jumpscare|PhotoScare|GetUseCustomPhotoScare)
                    (Utilities|👻PhotoScare👻-Custom (Variables|Settings|Jumpscare|PhotoScare|GetImage) (Variables|Settings|Jumpscare|Sound|GetSound) (Variables|Settings|Jumpscare|Additional|GetUseCameraShake) (Variables|Settings|Jumpscare|Additional|GetCameraShake)
                      (:Complete
                        (Actor|DestroyActor :!label _label_2)
                        (CallFunction|ActivateJumpscares))
                      (:Fail
                        (Development|PrintString "Photo Scare - Fail" true true "(R=1.000000,G=0.000000,B=0.036115,A=1.000000)" :!label _label_3)))
                    (else
                      (Utilities|👻PhotoScare👻 (Variables|Default|GetPhoto%20Scare%20DT)
                        (:Complete
                          (goto _label_2))
                        (:Fail
                          (goto _label_3)))))
                  (else
                    (bind _object (Utilities|AsyncLoadAsset (Variables|Settings|Jumpscare|Sound|GetSound) :!label _label_4)
                      (:Completed
                        (bind _assound_base (Utilities|Casting|CastToSoundBase _object)
                          (:then
                            (Audio|PlaySound2D _assound_base 1.0 1.0 0.0 0 0)
                            (Actor|DestroyActor))
                          (:CastFailed
                            _))
                        ;;[0 0 0] Jumpscare Camera Shake
                        (if (Variables|Settings|Jumpscare|Additional|GetUseCameraShake) :!label _label_5
                          (Class|LegacyCameraShake|StartLegacyCameraShake (Variables|/Script/Engine.PlayerController|GetPlayerCameraManager (Game|GetPlayerController 0)) (Variables|Settings|Jumpscare|Additional|GetCameraShake) 1.0 "CameraLocal" "0, 0, 0"))
                        (Actor|DestroyActor)
                        (CallFunction|ActivateJumpscares)))))
                (elif (Variables|Settings|Jumpscare|Sound|GetUseJumpscareSound)
                  (goto _label_4)
                  (elif (Variables|Settings|Jumpscare|PhotoScare|GetUsePhotoScare)
                    (bind _object_2 (Utilities|AsyncLoadAsset (Variables|Settings|Jumpscare|PhotoScare|GetImage))
                      (:Completed
                        (bind _astexture_2d (Utilities|Casting|CastToTexture2D _object_2)
                          (:then
                            (bind _returnvalue (UserInterface|CreateWidget "/Game/JumpscarePackX/Blueprints/Widgets/WB_Jumpscare_Screen.WB_Jumpscare_Screen_C" 0 _astexture_2d))
                            (UserInterface|Viewport|AddtoViewport _returnvalue 0)
                            (goto _label_5))
                          (:CastFailed
                            (goto _label_5)))))
                    (else
                      (goto _label_5)))))
              (else
                ;;[0 0 0] Actor
                (Variables|Settings|GetJumpscare
                  (:then
                    (if (Variables|Settings|Jumpscare|Additional|GetActivateJumpscareAfterRender)
                      (bind _returnvalue_2 (Utilities|Time|SetTimerbyEvent (delegate Custom|CustomEvent) 0.016 true))
                      (Variables|Don'tEdit|SetRenderCheckTimer _returnvalue_2)
                      (bind _returnvalue_3 (Utilities|Time|SetTimerbyEvent (delegate Custom|CustomEvent_0) (Variables|Settings|Jumpscare|Additional|GetMaxRenderCheckTime)))
                      (Variables|Don'tEdit|SetMaxRenderCheckTimer _returnvalue_3)
                      (else
                        (Default|Start (Variables|Settings|GetJumpscare) (Variables|Don'tEdit|GetData))
                        (Actor|DestroyActor))))
                  (:else
                    (CallFunction|ActivateJumpscares)
                    (goto _label)))))))))))

(event Custom|CustomEvent
  ;[0 0 0] Trigger Jumpscare
  ;;[0 0 0] Actor
  (if (Class|Actor|WasRecentlyRendered (Variables|Settings|GetJumpscare) 0.2)
    (Default|Start (Variables|Settings|GetJumpscare) (Variables|Don'tEdit|GetData))
    (Utilities|Time|ClearandInvalidateTimerbyHandle (Variables|Don'tEdit|GetRenderCheckTimer))
    (Utilities|Time|ClearandInvalidateTimerbyHandle (Variables|Don'tEdit|GetMaxRenderCheckTimer))
    (Actor|DestroyActor)))

(event Custom|CustomEvent_0
  ;[0 0 0] Trigger Jumpscare
  ;;[0 0 0] Actor
  (if (Variables|Settings|Jumpscare|Additional|GetTriggerJumpscareEvenIfNotRendered)
    (bind _jumpscare (Variables|Settings|GetJumpscare)
      (:then
        (Default|Start _jumpscare (Variables|Don'tEdit|GetData))
        (Utilities|Time|ClearandInvalidateTimerbyHandle (Variables|Don'tEdit|GetRenderCheckTimer))
        (Actor|DestroyActor))
      (:else))
    (else
      (CallFunction|ActivateJumpscares)
      (Utilities|Time|ClearandInvalidateTimerbyHandle (Variables|Don'tEdit|GetRenderCheckTimer))
      (Actor|DestroyActor))))

(event EventBeginPlay
  ;[0 0 0] Begin Play
  (CallFunction|SetCollision))

(fn ConstructionScript)

(fn SetCollision
  (bind _box (Variables|Default|GetBox))
  ;[0 0 0] Set Collision
  (Collision|SetCollisionEnabled _box "QueryOnly")
  (Collision|SetCollisionResponsetoAllChannels _box "ECR_Ignore")
  (Collision|SetCollisionResponsetoChannel _box "ECC_Pawn" "ECR_Overlap")
  (return))

(fn SetData
  (Variables|Don'tEdit|SetData (Utilities|Struct|MakeS_Jumpscare_Data (Variables|Settings|Jumpscare|Sound|GetUseDefaultSound) (Variables|Settings|Jumpscare|Additional|GetUseCameraShake) (Variables|Settings|Jumpscare|Additional|GetCameraShake) (Variables|Settings|Jumpscare|Sound|GetSound) (Variables|Settings|GetJumpscaresToActivate) (Variables|Settings|GetPrepareJumpscareActorsToActivate)))
  (return))

(fn ActivateJumpscares
  (bind _data (Variables|Don'tEdit|GetData))
  (bind (_usedefaultsound _usecamerashake _camerashake _sound _jumpscarestoactivate _preparejumpscareactorstoactivate) (Utilities|Struct|BreakS_Jumpscare_Data _data))
  ;[0 0 0] Active Jumpscares
  (for _array_element _jumpscarestoactivate
    (Utilities|IsValid _array_element
      (:Is%20Valid
        (Variables|BP_TriggerJumpscare_C|SetActive _array_element true))))
  (for _array_element_2 _preparejumpscareactorstoactivate
    (Utilities|IsValid _array_element_2
      (:Is%20Valid
        (Variables|/Game/JumpscarePackX/Blueprints/BP_PrepareJumpscare.BP_PrepareJumpscare_C|SetActive _array_element_2 true))))
  (return))