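; Interactable wine bottle puzzle piece that turns a quarter turn with a sound on each interaction.
; A timeline lerps the yaw, ignoring re-triggers mid-turn, then increments BottlePosition without wrapping and fires the puzzle-completed dispatcher when it equals PuzzleAnswer.
; Finalised gates interaction but is only set false here, so completion does not lock the bottle.
; Two overlap spheres swap outer and inner proximity icons, sized by the construction script.
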(event OnComponentBeginOverlap(InnerIconRadius)
  (params (OverlappedComponent :type Primitive%20Component%20Object%20Reference) (OtherActor :type Actor%20Object%20Reference) (OtherComp :type Primitive%20Component%20Object%20Reference) (OtherBodyIndex :type Integer) (bFromSweep :type Boolean) (SweepResult :type Hit%20Result%20Structure%20%28by%20ref%29))
  (if (== OtherActor (Game|GetPlayerCharacter 0))
    (Development|SetHiddeninGame (Variables|Default|GetInnerIcon) false false)
    (Development|SetHiddeninGame (Variables|Default|GetOuterIcon) true false)))

(event OnComponentEndOverlap(InnerIconRadius)
  (params (OverlappedComponent :type Primitive%20Component%20Object%20Reference) (OtherActor :type Actor%20Object%20Reference) (OtherComp :type Primitive%20Component%20Object%20Reference) (OtherBodyIndex :type Integer))
  (if (== (Game|GetPlayerCharacter 0) OtherActor)
    (Development|SetHiddeninGame (Variables|Default|GetInnerIcon) true false)
    (Development|SetHiddeninGame (Variables|Default|GetOuterIcon) false false)))

(event OnComponentBeginOverlap(OuterIconRadius)
  (params (OverlappedComponent :type Primitive%20Component%20Object%20Reference) (OtherActor :type Actor%20Object%20Reference) (OtherComp :type Primitive%20Component%20Object%20Reference) (OtherBodyIndex :type Integer) (bFromSweep :type Boolean) (SweepResult :type Hit%20Result%20Structure%20%28by%20ref%29))
  (if (== OtherActor (Game|GetPlayerCharacter 0))
    (Development|SetHiddeninGame (Variables|Default|GetOuterIcon) false false)))

(event OnComponentEndOverlap(OuterIconRadius)
  (params (OverlappedComponent :type Primitive%20Component%20Object%20Reference) (OtherActor :type Actor%20Object%20Reference) (OtherComp :type Primitive%20Component%20Object%20Reference) (OtherBodyIndex :type Integer))
  (if (== (Game|GetPlayerCharacter 0) OtherActor)
    (Development|SetHiddeninGame (Variables|Default|GetOuterIcon) true false)))

(event Custom|RotateBottle
  (if (not (Variables|Default|GetBottleMoving))
    (Variables|Default|SetBottleMoving true)
    (Audio|PlaySound2D "/Game/InteractionBlueprint/DiningRoomPuzzle/Audio/571138__dfsd32111__movepotion_Cue.571138__dfsd32111__movepotion_Cue" 1.0 1.0 0.0 0 0)
    (bind _alpha (Timeline|BottleRotation PlayFromStart)
      (:Update
        (Transformation|SetRelativeRotation (Variables|Default|GetWhine%20Bottle) (Math|Rotator|MakeRotator 0.0 0.0 (Math|Float|Lerp (.yaw (Variables|Default|GetStartingRotationBottle)) (- (.yaw (Variables|Default|GetStartingRotationBottle)) 9e+01) _alpha)) false false))
      (:Finished
        (Variables|Default|SetStartingRotationBottle (Math|Rotator|MakeRotator 0.0 0.0 (Math|Float|Lerp (.yaw (Variables|Default|GetStartingRotationBottle)) (- (.yaw (Variables|Default|GetStartingRotationBottle)) 9e+01) _alpha)))
        (Variables|Default|SetBottleMoving false)
        (bind _result (Math|Integer|IncrementInt (Variables|Default|GetBottlePosition))
          (:%20%20
            (Variables|Default|SetBottlePosition _result)
            (if (== (Variables|Default|GetPuzzleAnswer) (Variables|Default|GetBottlePosition))
              (Variables|Default|SetFinalised false)
              (Default|CallEVDPuzzleCompleted))))))))

(event EventBeginPlay
  (Variables|Default|SetStartingRotationBottle (Variables|/Script/Engine.SceneComponent|GetRelativeRotation (Variables|Default|GetWhine%20Bottle))))

(event EventInteraction
  (if (not (Variables|Default|GetFinalised))
    (CallFunction|RotateBottle)))

(fn ConstructionScript
  (Utilities|FlowControl|Sequence
    (:then_0
      (|CallParentFunction))
    (:then_1
      (Transformation|SetWorldScale3D (Variables|Default|GetInnerIcon) (Math|Conversions|ToVector(Float) (/ (Variables|Default|GetIconSize) 1e+01)))
      (Transformation|SetRelativeLocation (Variables|Default|GetInnerIcon) (Variables|Default|GetIconLocation) false false))
    (:then_2
      (Components|Sphere|SetSphereRadius (Variables|Default|GetInnerIconRadius) (Variables|Default|GetInnerRadius) true)
      (Components|Sphere|SetSphereRadius (Variables|Default|GetOuterIconRadius) (Variables|Default|GetOuterRadius) true))))