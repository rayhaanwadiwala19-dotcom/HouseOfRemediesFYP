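; Rotating goat statue puzzle that the player solves by interacting until the statue's position count matches PuzzleAnswer.
; Each interaction plays a metal sound and runs a timeline that yaws the statue by -90 degrees, ignoring input while it moves.
; When a turn ends, GoatPosition increments without wrapping; a match locks the puzzle, plays an unlock sound and calls the EVDPuzzleCompleted dispatcher.
; Tick prints GoatPosition on screen for debugging.
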(event Custom|RotateGoat
  (if (not (Variables|Default|GetGoatMoving))
    (Variables|Default|SetGoatMoving true)
    (Audio|PlaySound2D "/Game/InteractionBlueprint/WoodenBox/BoxStatuePuzzleSingular/Audio/MetalObjectMove_Cue.MetalObjectMove_Cue" 1.0 1.0 0.0 0 0)
    (bind _alpha (Timeline|GoatRotation PlayFromStart)
      (:Update
        (Transformation|SetRelativeRotation (Variables|Default|GetGoatStatue) (Math|Rotator|MakeRotator 0.0 0.0 (Math|Float|Lerp (.yaw (Variables|Default|GetStartingRotationGoat)) (- (.yaw (Variables|Default|GetStartingRotationGoat)) 9e+01) _alpha)) false false))
      (:Finished
        (Variables|Default|SetStartingRotationGoat (Math|Rotator|MakeRotator 0.0 0.0 (Math|Float|Lerp (.yaw (Variables|Default|GetStartingRotationGoat)) (- (.yaw (Variables|Default|GetStartingRotationGoat)) 9e+01) _alpha)))
        (Variables|Default|SetGoatMoving false)
        (bind _result (Math|Integer|IncrementInt (Variables|Default|GetGoatPosition))
          (:%20%20
            (Variables|Default|SetGoatPosition _result)
            (if (== (Variables|Default|GetPuzzleAnswer) (Variables|Default|GetGoatPosition))
              (Development|PrintString "PuzzleFinished" true true "(R=1.000000,G=0.749831,B=0.000000,A=1.000000)")
              (Variables|Default|SetFinalized true)
              (Audio|PlaySound2D "/Game/InteractionBlueprint/WoodenBox/Audio/UnlockedBox_Cue.UnlockedBox_Cue" 1.0 1.0 0.0 0 0)
              (Default|CallEVDPuzzleCompleted))))))))

(event EventBeginPlay
  (Variables|Default|SetStartingRotationGoat (Variables|/Script/Engine.SceneComponent|GetRelativeRotation (Variables|Default|GetGoatStatue))))

(event EventInteraction
  (if (not (Variables|Default|GetFinalized))
    (CallFunction|RotateGoat)))

(event EventTick
  (params (DeltaSeconds :type Float%20%28single-precision%29))
  (Development|PrintString (Utilities|String|ToString(Integer) (Variables|Default|GetGoatPosition)) true true "(R=0.000000,G=0.660000,B=1.000000,A=1.000000)" DeltaSeconds))

(fn ConstructionScript
  (|CallParentFunction))