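; Box trigger actor that fires the third jumpscare when the player character overlaps it, in one of two flag-selected modes.
; With Jumpscare1 set, it sends Jumpscare3Message to the referenced Actor on each overlap.
; Otherwise, Jumpscare2 plays a brief camera shake and a 2D sound, sends VisOnMessage to the player, then clears itself so that scare runs once.
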(event OnComponentBeginOverlap(Box)
  (params (OverlappedComponent :type Primitive%20Component%20Object%20Reference) (OtherActor :type Actor%20Object%20Reference) (OtherComp :type Primitive%20Component%20Object%20Reference) (OtherBodyIndex :type Integer) (bFromSweep :type Boolean) (SweepResult :type Hit%20Result%20Structure%20%28by%20ref%29))
  (bind _actor (Variables|Default|GetActor))
  (if (== OtherActor (Game|GetPlayerCharacter 0))
    (if (Variables|Default|GetJumpscare1)
      (Utilities|IsValid _actor
        (:Is%20Valid
          (Class|BPIJumpscare3|Jumpscare3(Message) _actor)))
      (elif (Variables|Default|GetJumpscare%202)
        (Class|LegacyCameraShake|StartLegacyCameraShake (Game|GetPlayerCameraManager 0) "/Game/JumpScares/JumpScare3/BP_JSShake.BP_JSShake_C" 2.0 "CameraLocal" "0, 0, 0")
        (Audio|PlaySound2D "/Game/JumpscarePackX/Audio/CUE/SC_Jumpscare3_Cue.SC_Jumpscare3_Cue" 1.0 1.0 0.0 0 0)
        (Class|BPIVisibility|Vison(Message) (Game|GetPlayerCharacter 0))
        (Utilities|FlowControl|Sequence
          (:then_0
            (Utilities|FlowControl|Delay 0.2)
            (Game|Feedback|ClientStopCameraShake (Game|GetPlayerController 0) "/Game/JumpScares/JumpScare3/BP_JSShake.BP_JSShake_C" true))
          (:then_1
            (Variables|Default|SetJumpscare%202 false)))))))

(event EventBeginPlay)

(event Collision|EventActorBeginOverlap
  (params (OtherActor :type Actor%20Object%20Reference)))

(event EventTick
  (params (DeltaSeconds :type Float%20%28single-precision%29)))

(fn ConstructionScript)