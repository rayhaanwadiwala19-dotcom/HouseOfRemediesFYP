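; BP_JSAI3 is a jumpscare AI pawn that rushes the player when they enter its Box trigger.
; On overlap with the player it destroys its Spotlight, plays a 2D jumpscare sound and starts the chase.
; The chase raises its custom time dilation for a sped-up run animation and uses AIMoveTo toward the player, destroying itself on success.
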(event OnComponentBeginOverlap(Box)
  (params (OverlappedComponent :type Primitive%20Component%20Object%20Reference) (OtherActor :type Actor%20Object%20Reference) (OtherComp :type Primitive%20Component%20Object%20Reference) (OtherBodyIndex :type Integer) (bFromSweep :type Boolean) (SweepResult :type Hit%20Result%20Structure%20%28by%20ref%29))
  (if (== OtherActor (Game|GetPlayerCharacter 0))
    (CallFunction|ChasePlayer)
    (Actor|DestroyActor (Variables|Default|GetSpotlight))
    (Audio|PlaySound2D "/Game/JumpScares/JumpScare1/Audio/Jumpscare_SFX.Jumpscare_SFX" 1.0 1.0 0.0 0 0)))

(event Custom|Chase%20Player
  (Variables|Default|SetCustomTimeDilation 5.0)
  (Components|Animation|PlayAnimation (Variables|Character|GetMesh) "/Game/Whisper/Animations/Anim_Whisper_Run.Anim_Whisper_Run" false)
  (AI|AIMoveTo self "0, 0, 0" (Game|GetPlayerCharacter 0) 5.0 false
    (:OnSuccess
      (Actor|DestroyActor))))

(event EventBeginPlay)

(fn ConstructionScript)