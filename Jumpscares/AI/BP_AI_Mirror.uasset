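; BP_AI_Mirror is a jumpscare AI actor that chases the player on demand and can be returned to its start.
; MoveToPlayer loops the mesh animation and runs AI MoveTo toward the player, firing OnSuccess on arrival.
; StopMoveandResetPosition halts movement and animation, then teleports it to the location cached at BeginPlay.
; Two cross-resetting DoOnce gates make the events alternate, ignoring repeated calls.
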(event Custom|Move%20To%20Player
  ;[0 0 0] Move / Stop
  (Utilities|FlowControl|Sequence
    (:then_0
      (Utilities|FlowControl|DoOnce false) ; enters at Reset
    )
    (:then_1
      (Utilities|FlowControl|DoOnce false
        (:Completed
          (Audio|Components|Audio|Play (Variables|Character|GetMesh) true)
          (AI|AIMoveTo self "0, 0, 0" (Game|GetPlayerCharacter 0) 5.0 false
            (:OnSuccess
              (Default|CallOnSuccess))))))))

(event Custom|Stop%20Move%20and%20Reset%20Position
  ;[0 0 0] Move / Stop
  (Utilities|FlowControl|Sequence
    (:then_0
      (Utilities|FlowControl|DoOnce false) ; enters at Reset
    )
    (:then_1
      (Utilities|FlowControl|DoOnce false
        (:Completed
          (AI|Navigation|StopMovement (AI|GetAIController self))
          (Audio|Components|Audio|Stop (Variables|Character|GetMesh))
          (Transformation|SetActorLocation (Variables|Default|GetStart%20Location) false false))))))

(event EventBeginPlay
  ;[0 0 0] Begin Play
  (Variables|Default|SetStart%20Location (Transformation|GetActorLocation)))

(fn ConstructionScript)