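; Jumpscare actor that reveals a hidden animated character and reacts once the player has it in view.
; PrepareJumpscare async-loads the idle animation, hide montage, mesh and AnimBP in sequence; triggering retries on a capped timer until they are ready.
; Once revealed, Tick uses WasRecentlyRendered on a sphere to detect visibility, then fires sound and camera shake.
; After a delay it plays the hide montage and destroys itself.
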(event Custom|CustomEvent
  ;[0 0 0] Trigger Jumpscare
  (Animation|Montage|PlayMontage (Variables|Default|GetSkeletalMesh) (Variables|Don'tEdit|GetHide%20-%20Loaded)
    (:OnCompleted
      _)
    (:OnBlendOut
      _)
    (:OnInterrupted
      _))
  (Actor|DestroyActor))

(event Custom|CustomEvent_0
  ;[0 0 0] Trigger Jumpscare
  (Utilities|FlowControl|DoN 15
    (:Exit
      (if (Variables|Don'tEdit|GetPrepared)
        (Development|SetHiddeninGame (Variables|Default|GetSkeletalMesh) false false)
        (Utilities|FlowControl|Delay 0.2)
        (Actor|Tick|SetActorTickEnabled true)
        (else
          (Utilities|Time|SetTimerbyEvent (delegate Custom|CustomEvent_0) 0.5))))))

(event EventPrepareJumpscare
  ;[0 0 0] Preload
  (Utilities|FlowControl|DoOnce false
    (:Completed
      (bind _object (Utilities|AsyncLoadAsset (Variables|Settings|GetIdle))
        (:Completed
          (bind _asanim_sequence (Utilities|Casting|CastToAnimSequence _object))
          (Variables|Don'tEdit|SetIdle%20-%20Loaded _asanim_sequence)
          (bind _object_2 (Utilities|AsyncLoadAsset (Variables|Settings|GetHide%20-%20Montage))
            (:Completed
              (bind _asanim_montage (Utilities|Casting|CastToAnimMontage _object_2))
              (Variables|Don'tEdit|SetHide%20-%20Loaded _asanim_montage)
              (bind _object_3 (Utilities|AsyncLoadAsset (Variables|Settings|GetSkeletal%20Mesh))
                (:Completed
                  (bind _asskeletal_mesh (Utilities|Casting|CastToSkeletalMesh _object_3))
                  (Variables|/Script/Engine.SkeletalMeshComponent|SetSkeletalMeshAsset (Variables|Default|GetSkeletalMesh) _asskeletal_mesh)
                  (bind _class (Utilities|AsyncLoadClassAsset (Variables|Settings|GetAnim%20BP))
                    (:Completed
                      (bind _asanim_instance (Utilities|Casting|CastToAnimInstanceClass _class))
                      (Class|SkeletalMeshComponent|SetAnimClass (Variables|Default|GetSkeletalMesh) _asanim_instance)
                      (Class|BPIJumpscarePackX|SetAnimation(Message) (Components|SkeletalMesh|GetAnimInstance (Variables|Default|GetSkeletalMesh)) (Variables|Don'tEdit|GetIdle%20-%20Loaded))
                      (Variables|Don'tEdit|SetPrepared true))))))))))))

(event EventTriggerJumpscare
  ;[0 0 0] Trigger Jumpscare
  (if (Variables|Don'tEdit|GetPrepared)
    (Development|SetHiddeninGame (Variables|Default|GetSkeletalMesh) false false)
    (Utilities|FlowControl|Delay 0.2)
    (Actor|Tick|SetActorTickEnabled true)
    (else
      (Utilities|Time|SetTimerbyEvent (delegate Custom|CustomEvent_0) 0.5))))

(event EventTick
  (params (DeltaSeconds :type Float%20%28single-precision%29))
  ;[0 0 0] Trigger Jumpscare
  (if (Class|PrimitiveComponent|WasRecentlyRendered (Variables|Default|GetSphere) 0.2)
    (Utilities|FlowControl|DoOnce false
      (:Completed
        (CallFunction|SpawnSound)
        (CallFunction|PlayCameraShake)
        (Actor|Tick|SetActorTickEnabled false)
        (Utilities|Time|SetTimerbyEvent (delegate Custom|CustomEvent) (Variables|Settings|GetDelay%20Before%20Hide))))))

(fn ConstructionScript
  (|CallParentFunction)
  (if (Variables|Settings|GetReady)
    (Components|DestroyComponent (Variables|Default|GetSkeletalMesh1))))