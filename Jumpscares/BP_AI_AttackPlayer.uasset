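; Jumpscare actor that spawns an AI character and sends it charging at the player.
; Preparation runs once, async-loading the idle and attack animations and character class, then spawning the character idling at the Spawn point.
; Triggering plays the attack animation and moves the AI to the player, retrying on a timer if not ready.
; Whether the move succeeds or fails, it runs StartShockLink with camera data, then destroys the character.
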(event Custom|CustomEvent
  (bind _character (Variables|Don'tEdit|GetCharacter))
  (bind _mesh (Variables|/Script/Engine.Character|GetMesh _character))
  ;[0 0 0] Trigger Jumpscare
  (if (Variables|Don'tEdit|GetReady)
    (Components|Animation|PlayAnimation _mesh (Variables|Don'tEdit|GetAttack%20Anim%20-%20Loaded) true)
    (Components|Timeline|SetPlayRate _mesh (Variables|Settings|GetAnimation%20Play%20Rate))
    (AI|AIMoveTo (Variables|Don'tEdit|GetCharacter) "0, 0, 0" (Game|GetPlayerCharacter 0) 5.0 false
      (:OnSuccess
        _)
      (:OnFail
        _))
    (Utilities|👻StartShockLink👻 (Variables|Settings|GetCameraData)
      (:Completed
        (Actor|DestroyActor (Variables|Don'tEdit|GetCharacter))))
    (else
      (CallFunction|PrepareJumpscare)
      (Utilities|Time|SetTimerbyEvent (delegate Custom|CustomEvent) 0.5))))

(event EventTriggerJumpscare
  (bind _character (Variables|Don'tEdit|GetCharacter))
  (bind _mesh (Variables|/Script/Engine.Character|GetMesh _character))
  ;[0 0 0] Trigger Jumpscare
  (if (Variables|Don'tEdit|GetReady)
    (Components|Animation|PlayAnimation _mesh (Variables|Don'tEdit|GetAttack%20Anim%20-%20Loaded) true)
    (Components|Timeline|SetPlayRate _mesh (Variables|Settings|GetAnimation%20Play%20Rate))
    (AI|AIMoveTo (Variables|Don'tEdit|GetCharacter) "0, 0, 0" (Game|GetPlayerCharacter 0) 5.0 false
      (:OnSuccess
        _)
      (:OnFail
        _))
    (Utilities|👻StartShockLink👻 (Variables|Settings|GetCameraData)
      (:Completed
        (Actor|DestroyActor (Variables|Don'tEdit|GetCharacter))))
    (else
      (CallFunction|PrepareJumpscare)
      (Utilities|Time|SetTimerbyEvent (delegate Custom|CustomEvent) 0.5))))

(event EventPrepareJumpscare
  ;[0 0 0] Prepare Jumpscare
  (Utilities|FlowControl|DoOnce false
    (:Completed
      (bind _object (Utilities|AsyncLoadAsset (Variables|Settings|GetIdleAnimation))
        (:Completed
          (bind _asanim_sequence (Utilities|Casting|CastToAnimSequence _object))
          (Variables|Don'tEdit|SetIdle%20Anim%20-%20Loaded _asanim_sequence)
          (bind _object_2 (Utilities|AsyncLoadAsset (Variables|Settings|GetAttackAnimation))
            (:Completed
              (bind _asanim_sequence_2 (Utilities|Casting|CastToAnimSequence _object_2))
              (Variables|Don'tEdit|SetAttack%20Anim%20-%20Loaded _asanim_sequence_2)
              (bind _class (Utilities|AsyncLoadClassAsset (Variables|Settings|GetAI%20Class))
                (:Completed
                  (bind _ascharacter (Utilities|Casting|CastToCharacterClass _class))
                  (bind _returnvalue (Game|SpawnActorfromClass _ascharacter (Math|Transform|MakeTransform (Transformation|GetWorldLocation (Variables|Default|GetSpawn)) (Transformation|GetWorldRotation (Variables|Default|GetSpawn1)) "1.000000,1.000000,1.000000") "Undefined" "MultiplyWithRoot" 0 0))
                  (Variables|/Script/Engine.CharacterMovementComponent|SetMaxWalkSpeed (Actor|GetComponentbyClass _returnvalue "/Script/Engine.CharacterMovementComponent") (Variables|Settings|GetMax%20Walk%20Speed))
                  (bind _output_get (Variables|Don'tEdit|SetCharacter _returnvalue))
                  (Components|Animation|PlayAnimation (Variables|/Script/Engine.Character|GetMesh _output_get) (Variables|Don'tEdit|GetIdle%20Anim%20-%20Loaded) true)
                  (Variables|Don'tEdit|SetReady true))))))))))

(fn ConstructionScript)