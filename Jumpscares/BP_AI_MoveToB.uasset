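; Jumpscare actor that spawns a character at point A and walks it to point B with a looping animation and a sound, then destroys it.
; PrepareJumpscare async-loads the class and spawns the character once with a set walk speed.
; Triggering retries on a 0.5s timer through an event that also runs the preload, until ready.
; The construction script spaces A and B symmetrically along local X from one distance value.
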(event Custom|CustomEvent
  (bind _character (Variables|Don'tEdit|GetCharacter))
  (bind _mesh (Variables|/Script/Engine.Character|GetMesh _character))
  ;[0 0 0] Trigger Jumpscare
  (CallFunction|PrepareJumpscare)
  (if (Variables|Don'tEdit|GetReady)
    (CallFunction|SpawnSound)
    (Components|Animation|PlayAnimation _mesh (Variables|Settings|GetWalk%20Anim%20Seq) true)
    (Components|Timeline|SetPlayRate _mesh (Variables|Settings|GetAnimation%20Play%20Rate))
    (AI|AIMoveTo (Variables|Don'tEdit|GetCharacter) (Transformation|GetWorldLocation (Variables|Default|GetB)) 0 5.0 false
      (:OnSuccess
        _)
      (:OnFail
        _))
    (Actor|DestroyActor (Variables|Don'tEdit|GetCharacter))
    (else
      (Utilities|Time|SetTimerbyEvent (delegate Custom|CustomEvent) 0.5))))

(event EventTriggerJumpscare
  (bind _character (Variables|Don'tEdit|GetCharacter))
  (bind _mesh (Variables|/Script/Engine.Character|GetMesh _character))
  ;[0 0 0] Trigger Jumpscare
  (if (Variables|Don'tEdit|GetReady)
    (CallFunction|SpawnSound)
    (Components|Animation|PlayAnimation _mesh (Variables|Settings|GetWalk%20Anim%20Seq) true)
    (Components|Timeline|SetPlayRate _mesh (Variables|Settings|GetAnimation%20Play%20Rate))
    (AI|AIMoveTo (Variables|Don'tEdit|GetCharacter) (Transformation|GetWorldLocation (Variables|Default|GetB)) 0 5.0 false
      (:OnSuccess
        _)
      (:OnFail
        _))
    (Actor|DestroyActor (Variables|Don'tEdit|GetCharacter))
    (else
      (Utilities|Time|SetTimerbyEvent (delegate Custom|CustomEvent) 0.5))))

(event EventPrepareJumpscare
  ;[0 0 0] Jumpscare Preload
  (Utilities|FlowControl|DoOnce false
    (:Completed
      (bind _class (Utilities|AsyncLoadClassAsset (Variables|Settings|GetAI%20Class))
        (:Completed
          (bind _ascharacter (Utilities|Casting|CastToCharacterClass _class))
          (bind _returnvalue (Game|SpawnActorfromClass _ascharacter (Math|Transform|MakeTransform (Transformation|GetWorldLocation (Variables|Default|GetA)) "0, 0, 0" "1.000000,1.000000,1.000000") "Undefined" "MultiplyWithRoot" 0 0))
          (Variables|/Script/Engine.CharacterMovementComponent|SetMaxWalkSpeed (Actor|GetComponentbyClass _returnvalue "/Script/Engine.CharacterMovementComponent") (Variables|Settings|GetMax%20Walk%20Speed))
          (Variables|Don'tEdit|SetCharacter _returnvalue)
          (Variables|Don'tEdit|SetReady true))))))

(fn ConstructionScript
  (bind _distancebetweenab (Variables|Settings|GetDistanceBetweenAB))
  (bind _returnvalue (/ _distancebetweenab 2.0))
  (Transformation|SetRelativeLocation (Variables|Default|GetB) (Math|Vector|MakeVector _returnvalue 0.0 9e+01) false false)
  (Transformation|SetRelativeLocation (Variables|Default|GetA) (Math|Vector|MakeVector (* _returnvalue -1.0) 0.0 9e+01) false false))