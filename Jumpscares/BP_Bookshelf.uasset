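; Bookshelf jumpscare actor that, when triggered, throws its books off while playing a sound and camera shake.
; Book meshes ignore collision from BeginPlay, then LaunchBooks enables physics, blocks only world static and pushes them using an arrow component and FallForce.
; A timeline tilts the shelf mesh during the scare.
; Five seconds after the trigger, a timer turns off the books' physics and collision.
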(event Custom|CustomEvent
  ;[0 0 0] Trigger
  (for _array_element (Variables|Default|GetAs%20Static%20Mesh%20Component%20X)
    (Physics|SetSimulatePhysics _array_element false)
    (Collision|SetCollisionEnabled _array_element "NoCollision")))

(event EventBeginPlay
  ;[0 0 0] Begin Play
  (|CallParentFunction)
  (CallFunction|SetCollision))

(event EventTriggerJumpscare
  ;[0 0 0] Trigger
  (CallFunction|LaunchBooks)
  (CallFunction|SpawnSound)
  (CallFunction|PlayCameraShake)
  (Utilities|Time|SetTimerbyEvent (delegate Custom|CustomEvent) 5.0)
  (bind _alphax (Timeline|Timeline PlayFromStart)
    (:Update
      (Transformation|SetRelativeRotation (Variables|Default|GetStaticMesh) (Math|Rotator|Lerp(Rotator) "0, 0, 0" "0.000000,0.000000,7.000000" _alphax) false false))))

(fn ConstructionScript
  (|CallParentFunction))

(fn SetCollision
  (for _array_element (Components|GetChildrenComponents (Variables|Default|GetBooks) false)
    (bind _asstatic_mesh_component (Utilities|Casting|CastToStaticMeshComponent _array_element))
    (Collision|SetCollisionResponsetoAllChannels _asstatic_mesh_component "ECR_Ignore"))
  (return))

(fn LaunchBooks
  (bind _arrow (Variables|Default|GetArrow))
  ;[0 0 0] Launch Books
  (LocalVariables|SetBooks%20L (Components|GetChildrenComponents (Variables|Default|GetBooks) false))
  (for _array_element (LocalVariables|GetBooks%20L)
    (bind _asstatic_mesh_component (Utilities|Casting|CastToStaticMeshComponent _array_element))
    (Utilities|Array|Add (Variables|Default|GetAs%20Static%20Mesh%20Component%20X) _asstatic_mesh_component)
    (Physics|SetSimulatePhysics _asstatic_mesh_component true)
    (Physics|AddForce _asstatic_mesh_component (+ (Transformation|GetWorldLocation _arrow) (* (Math|Vector|GetForwardVector _arrow) (Variables|Settings|GetFall%20Force))) "None" false)
    (Collision|SetCollisionEnabled _asstatic_mesh_component "PhysicsOnly")
    (Collision|SetCollisionResponsetoChannel _asstatic_mesh_component "ECC_WorldStatic" "ECR_Block")
    (Collision|SetCollisionResponsetoChannel _asstatic_mesh_component "ECC_WorldDynamic" "ECR_Ignore"))
  (return))