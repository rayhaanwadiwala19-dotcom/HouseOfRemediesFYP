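; Base jumpscare actor that runs a scare from a data struct and exposes empty trigger, prepare and toggle-active events, apparently for child Blueprints.
; Start fires once, async-loading the default or custom soft-referenced sound before calling TriggerJumpscare.
; It then activates linked jumpscare and prepare actors, allowing scares to be chained.
; Separate helper events play the sound at the actor's location and an optional camera shake on the first player.
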(event Custom|TriggerJumpscare
  ;[0 0 0] Trigger Jumpscare
)

(event Custom|Start
  (params (S_Jumpscare_Data :type S%20Jumpscare%20Data%20Structure%20%28by%20ref%29))
  (bind (_usedefaultsound _usecamerashake _camerashake _sound) (Utilities|Struct|BreakS_Jumpscare_Data S_Jumpscare_Data))
  (bind _default_sound (Variables|Settings|GetDefault%20Sound))
  ;[0 0 0] Jumpscare Data
  (Utilities|FlowControl|DoOnce false
    (:Completed
      (Variables|Default|SetS%20Jumpscare%20Data S_Jumpscare_Data)
      (if _usecamerashake
        _
        (else
          _))
      (if _usedefaultsound
        (if (Utilities|IsValidSoftObjectReference _default_sound)
          (bind _object (Utilities|AsyncLoadAsset _default_sound)
            (:Completed
              (bind _assound_base (Utilities|Casting|CastToSoundBase _object)
                (:then
                  (Variables|Default|SetJumpscare%20Sound _assound_base)
                  (CallFunction|TriggerJumpscare))
                (:CastFailed
                  (CallFunction|TriggerJumpscare :!label _label)))))
          (else
            (goto _label)))
        (CallFunction|ActivateJumpscares)
        (elif (Utilities|IsValidSoftObjectReference _sound)
          (bind _object_2 (Utilities|AsyncLoadAsset _sound)
            (:Completed
              (bind _assound_base_2 (Utilities|Casting|CastToSoundBase _object_2))
              (Variables|Default|SetJumpscare%20Sound _assound_base_2)
              (CallFunction|TriggerJumpscare)
              (CallFunction|ActivateJumpscares)))
          (else
            (CallFunction|TriggerJumpscare)
            (CallFunction|ActivateJumpscares)))))))

(event Custom|Spawn%20Sound
  ;[0 0 0] Spawn Sound
  (bind _jumpscare_sound (Variables|Default|GetJumpscare%20Sound)
    (:then
      (Audio|SpawnSoundatLocation _jumpscare_sound (Transformation|GetActorLocation) "0, 0, 0" 1.0 1.0 0.0 (Variables|Default|GetAttenuation%20Settings) 0))
    (:else)))

(event Custom|PrepareJumpscare
  ;[0 0 0] JumpscarePreload
)

(event Custom|Play%20Camera%20Shake
  (bind _s_jumpscare_data (Variables|Default|GetS%20Jumpscare%20Data))
  ;[0 0 0] Camera Shake
  (if (.usecamerashake _s_jumpscare_data)
    (Class|LegacyCameraShake|StartLegacyCameraShake (Variables|/Script/Engine.PlayerController|GetPlayerCameraManager (Game|GetPlayerController 0)) (.camerashake _s_jumpscare_data) 1.0 "CameraLocal" "0, 0, 0")))

(event Custom|ToggleActorActive
  (params (Active :type Boolean))
  ;[0 0 0] Toggle Actor Active
)

(fn ConstructionScript)

(fn ActivateJumpscares
  (bind _s_jumpscare_data (Variables|Default|GetS%20Jumpscare%20Data))
  (bind (_usedefaultsound _usecamerashake _camerashake _sound _jumpscarestoactivate _preparejumpscareactorstoactivate) (Utilities|Struct|BreakS_Jumpscare_Data _s_jumpscare_data))
  ;[0 0 0] Active Jumpscares
  (for _array_element _jumpscarestoactivate
    (Utilities|IsValid _array_element
      (:Is%20Valid
        (Variables|/Game/JumpscarePackX/Blueprints/BP_TriggerJumpscare.BP_TriggerJumpscare_C|SetActive _array_element true))))
  (for _array_element_2 _preparejumpscareactorstoactivate
    (Utilities|IsValid _array_element_2
      (:Is%20Valid
        (Variables|/Game/JumpscarePackX/Blueprints/BP_PrepareJumpscare.BP_PrepareJumpscare_C|SetActive _array_element_2 true))))
  (return))