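; Mirror jumpscare actor that renders a fake reflection via scene capture to a runtime render target, rotating it within clamped angles from the player camera.
; While one probe sphere is rendered and the other is not, an AI spawned below the arrow approaches the player; otherwise it hides and resets.
; AI success or a further sighting after the show limit destroys it and starts the shock link.
; ToggleActorActive switches tick and capture.
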(event Custom|CustomEvent
  ;[0 0 0] Spawn AI if the jumpscare is ready
  (Variables|Don'tEdit|SetEnd true)
  (bind _spawned_ai (Variables|Don'tEdit|GetSpawned%20AI)
    (:then
      (Actor|DestroyActor _spawned_ai)
      (Utilities|👻StartShockLink👻 (Variables|Settings|GetCameraData)))
    (:else)))

(event EventTriggerJumpscare
  ;[0 0 0] Trigger Jumpscare
)

(event EventPrepareJumpscare
  ;[0 0 0] Prepare
  (Utilities|FlowControl|DoOnce false))

(event EventTick
  (params (DeltaSeconds :type Float%20%28single-precision%29))
  (bind _returnvalue (Transformation|GetActorTransform))
  (bind _returnvalue_2 (Game|GetPlayerController 0))
  (bind _scenecapturecomponent2d (Variables|Default|GetSceneCaptureComponent2D))
  (bind _arrow (Variables|Default|GetArrow))
  (bind _returnvalue_3 (Transformation|GetWorldLocation _scenecapturecomponent2d))
  (bind _returnvalue_4 (Transformation|GetWorldLocation _arrow))
  (bind _playercameramanager (Variables|/Script/Engine.PlayerController|GetPlayerCameraManager _returnvalue_2))
  (bind _returnvalue_5 (Transformation|GetActorLocation _playercameramanager))
  (bind _returnvalue_6 (Transformation|GetActorForwardVector _playercameramanager))
  (bind _returnvalue_7 (* _returnvalue_6 -555.0))
  (bind _returnvalue_8 (+ _returnvalue_5 _returnvalue_7))
  (bind _returnvalue_9 (Math|Rotator|FindLookatRotation _returnvalue_3 _returnvalue_8))
  (bind _returnvalue_10 (* _returnvalue_9 -1.0))
  (bind _returnvalue_11 (Math|Transform|InverseTransformRotation _returnvalue _returnvalue_10))
  (bind (_roll _pitch _yaw) (Math|Rotator|BreakRotator _returnvalue_11))
  ;[0 0 0] Mirror Logic
  (Utilities|FlowControl|Sequence
    (:then_0
      ;[0 0 0] Spawn AI if the jumpscare is ready
      (if (not (Variables|Don'tEdit|GetEnd))
        (if (and (Class|PrimitiveComponent|WasRecentlyRendered (Variables|Default|GetSphere) 0.05) (not (Class|PrimitiveComponent|WasRecentlyRendered (Variables|Default|GetSphere1) 0.05)))
          (if (>= (Variables|Don'tEdit|GetCounter) (Variables|Settings|GetMaxAIShowTimes))
            (bind _spawned_ai (Variables|Don'tEdit|GetSpawned%20AI)
              (:then
                (Actor|DestroyActor _spawned_ai)
                (Utilities|👻StartShockLink👻 (Variables|Settings|GetCameraData)
                  (:Completed
                    (CallFunction|PlayCameraShake))))
              (:else))
            (else
              (Utilities|FlowControl|Sequence
                (:then_0
                  (Variables|Don'tEdit|GetSpawned%20AI
                    (:then
                      (Rendering|SetActorHiddenInGame (Variables|Don'tEdit|GetSpawned%20AI) false :!label _label)
                      (Default|MovetoPlayer (Variables|Don'tEdit|GetSpawned%20AI)))
                    (:else
                      (bind (_outhit _returnvalue_12) (Collision|LineTraceByChannel _returnvalue_4 (- _returnvalue_4 "0.000000,0.000000,555.000000") "TraceTypeQuery1" false 0 "None"))
                      (if _returnvalue_12
                        (bind _returnvalue_13 (Game|SpawnActorfromClass (Variables|Settings|GetAI%20Class) (Math|Transform|MakeTransform (.Location (Collision|BreakHitResult _outhit)) "0, 0, 0" "1.000000,1.000000,1.000000") "AdjustIfPossibleButAlwaysSpawn" "MultiplyWithRoot" 0 0))
                        (bind _output_get (Variables|Don'tEdit|SetSpawned%20AI _returnvalue_13))
                        (EventDispatchers|BindEventtoOnSuccess _output_get (delegate Custom|CustomEvent))
                        (goto _label)))))
                (:then_1
                  (Utilities|FlowControl|DoOnce true :!label _label_2
                    (:Completed
                      (Math|Integer|IncrementInt (Variables|Don'tEdit|GetCounter))))))))
          (else
            (bind _spawned_ai_2 (Variables|Don'tEdit|GetSpawned%20AI)
              (:then
                (Rendering|SetActorHiddenInGame _spawned_ai_2 true)
                (Default|StopMoveandResetPosition (Variables|Don'tEdit|GetSpawned%20AI))
                (goto _label_2 Reset))
              (:else))))))
    (:then_1
      (Transformation|SetRelativeRotation (Variables|Default|GetSceneCaptureComponent2D) (Math|Rotator|MakeRotator 0.0 (Math|Float|Clamp(Float) _pitch -45.0 45.0) (+ (Math|Float|Clamp(Float) _yaw -45.0 45.0) 9e+01)) false false))))

(event EventBeginPlay
  (bind _scenecapturecomponent2d (Variables|Default|GetSceneCaptureComponent2D))
  ;[0 0 0] Hide Actor Components For Scene Capture
  (Class|SceneCaptureComponent|HideActorComponents (Variables|Default|GetSceneCaptureComponent2D) self false)
  (bind _returnvalue (Rendering|CreateRenderTarget2D 1024 1024 "RTF_RGBA16f"))
  (bind _output_get (Variables|/Script/Engine.SceneCaptureComponent2D|SetTextureTarget _scenecapturecomponent2d _returnvalue))
  (Components|Activation|SetActive _scenecapturecomponent2d false false)
  (bind _returnvalue_2 (Rendering|Material|CreateDynamicMaterialInstance (Variables|Default|GetPlane) 0 (Rendering|Material|GetMaterial (Variables|Default|GetPlane) 0) "None" :!class /Script/Engine.PrimitiveComponent))
  (Rendering|Material|SetTextureParameterValue _returnvalue_2 "Render" _output_get)
  (Rendering|SetVisibility (Variables|Default|GetSphere1) true false))

(event EventToggleActorActive
  (params (Active :type Boolean))
  (bind _scenecapturecomponent2d (Variables|Default|GetSceneCaptureComponent2D))
  ;[0 0 0] Toggle Actor
  (Actor|Tick|SetActorTickEnabled Active)
  (Components|Activation|SetActive _scenecapturecomponent2d Active false)
  (Components|Tick|SetComponentTickEnabled _scenecapturecomponent2d Active))

(fn ConstructionScript
  (|CallParentFunction)
  (Transformation|SetRelativeLocation (Variables|Default|GetArrow) (Variables|Settings|GetAI%20Spawn%20Location) false false))