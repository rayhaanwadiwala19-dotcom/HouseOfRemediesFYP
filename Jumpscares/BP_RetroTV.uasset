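; Retro TV jumpscare that bursts its screen and plays an animated scare with sound and camera shake.
; When triggered, it async-loads montage, mesh and AnimBP, polls until ready, then spawns and attaches a BP_RetroTV_AI actor to play the montage.
; A looping timer randomly jumps to the End section; blend-out destroys the actor.
; Glass shards launch with physics, frozen after a delay, or are removed at BeginPlay when Optimized.
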(event Custom|CustomEvent_1
  ;[0 0 0] Trigger
  ;;[0 0 0] Physics / Collision - Glass
  (for _array_element (Variables|Don'tEdit|GetAs%20Static%20Mesh%20Component)
    (Physics|SetSimulatePhysics _array_element false)
    (Collision|SetCollisionEnabled _array_element "NoCollision")
    (Components|Activation|SetActive (Variables|Default|GetNiagara) false false)))

(event Custom|CustomEvent_0
  ;[0 0 0] Trigger
  ;;[0 0 0] Wait until the jumpscare is ready
  (if (Variables|Don'tEdit|GetReady)
    (bind _staticmesh1 (Variables|Default|GetStaticMesh1)
      (:then
        (Components|DestroyComponent _staticmesh1)
        (bind _returnvalue (Game|SpawnActorfromClass "/Game/JumpscarePackX/Blueprints/Jumpscares/AI/BP_RetroTV_AI.BP_RetroTV_AI_C" (Math|Transform|MakeTransform "0, 0, 0" "0.000000,-90.000000,0.000000" "1.000000,1.000000,1.000000") "AlwaysSpawn" "MultiplyWithRoot" 0 0))
        (Variables|Don'tEdit|SetRetro%20TV%20AI _returnvalue)
        (Variables|Don'tEdit|SetSkeletal%20Mesh%20Comp (Variables|/Game/JumpscarePackX/Blueprints/Jumpscares/AI/BP_RetroTV_AI.BP_RetroTV_AI_C|GetSkeletalMesh _returnvalue))
        (Transformation|AttachComponentToComponent _returnvalue (Variables|Default|GetArrow) "None" "KeepRelative" "KeepRelative" "KeepRelative" true)
        (Components|Activation|SetActive (Variables|Default|GetNiagara) true false)
        (bind _output_get (Variables|Default|SetSkeletal%20Mesh%20Component (Variables|Don'tEdit|GetSkeletal%20Mesh%20Comp)))
        (Components|SkeletalMesh|SetSkeletalMeshAsset _output_get (Variables|LoadedAssets|GetSkeletalMesh%20-%20Loaded))
        ;;[0 0 0] Start
        (Components|Animation|SetAnimationMode (Variables|Don'tEdit|GetSkeletal%20Mesh%20Comp) "AnimationBlueprint" true)
        (Class|SkeletalMeshComponent|SetAnimClass (Variables|Don'tEdit|GetSkeletal%20Mesh%20Comp) (Variables|LoadedAssets|GetAnimBP_Class%20-%20Loaded))
        (Animation|Montage|PlayMontage (Variables|Default|GetSkeletal%20Mesh%20Component) "/Game/JumpscarePackX/Animations/AM_RetroTV_Jumpscare_Start_Montage.AM_RetroTV_Jumpscare_Start_Montage"
          (:then
            (CallFunction|LaunchGlass)
            (CallFunction|SpawnSound)
            (CallFunction|PlayCameraShake)
            (bind _returnvalue_2 (Utilities|Time|SetTimerbyEvent (delegate Custom|CustomEvent) 1.0 true))
            (Variables|Don'tEdit|SetLoop%20-%20Timer _returnvalue_2)
            ;;[0 0 0] Physics / Collision - Glass
            (Utilities|Time|SetTimerbyEvent (delegate Custom|CustomEvent_1) 5.0))
          (:OnBlendOut
            ;;[0 0 0] Destroy Mesh
            (Actor|DestroyActor (Variables|Don'tEdit|GetRetro%20TV%20AI)))))
      (:else))
    (else
      (Utilities|Time|SetTimerbyEvent (delegate Custom|CustomEvent_0) 0.1))))

(event Custom|CustomEvent
  (bind _skeletal_mesh_component (Variables|Default|GetSkeletal%20Mesh%20Component))
  (bind _returnvalue (Components|SkeletalMesh|GetAnimInstance _skeletal_mesh_component))
  ;[0 0 0] Trigger
  ;;[0 0 0] End
  (if (Math|Random|RandomBool)
    (Ability|Animation|MontageJumptoSection _returnvalue "End" (Animation|Montage|GetCurrentActiveMontage _returnvalue))
    (Utilities|Time|ClearandInvalidateTimerbyHandle (Variables|Don'tEdit|GetLoop%20-%20Timer))))

(event EventBeginPlay
  ;[0 0 0] Begin Play
  (if (Variables|Settings|GetOptimized)
    (CallFunction|DestroyGlass (Components|GetChildrenComponents (Variables|Default|GetDestroyedScreen) false))))

(event EventTriggerJumpscare
  ;[0 0 0] Trigger
  (CallFunction|PrepareJumpscare)
  ;;[0 0 0] Wait until the jumpscare is ready
  (if (Variables|Don'tEdit|GetReady)
    (bind _staticmesh1 (Variables|Default|GetStaticMesh1)
      (:then
        (Components|DestroyComponent _staticmesh1)
        (bind _returnvalue (Game|SpawnActorfromClass "/Game/JumpscarePackX/Blueprints/Jumpscares/AI/BP_RetroTV_AI.BP_RetroTV_AI_C" (Math|Transform|MakeTransform "0, 0, 0" "0.000000,-90.000000,0.000000" "1.000000,1.000000,1.000000") "AlwaysSpawn" "MultiplyWithRoot" 0 0))
        (Variables|Don'tEdit|SetRetro%20TV%20AI _returnvalue)
        (Variables|Don'tEdit|SetSkeletal%20Mesh%20Comp (Variables|/Game/JumpscarePackX/Blueprints/Jumpscares/AI/BP_RetroTV_AI.BP_RetroTV_AI_C|GetSkeletalMesh _returnvalue))
        (Transformation|AttachComponentToComponent _returnvalue (Variables|Default|GetArrow) "None" "KeepRelative" "KeepRelative" "KeepRelative" true)
        (Components|Activation|SetActive (Variables|Default|GetNiagara) true false)
        (bind _output_get (Variables|Default|SetSkeletal%20Mesh%20Component (Variables|Don'tEdit|GetSkeletal%20Mesh%20Comp)))
        (Components|SkeletalMesh|SetSkeletalMeshAsset _output_get (Variables|LoadedAssets|GetSkeletalMesh%20-%20Loaded))
        ;;[0 0 0] Start
        (Components|Animation|SetAnimationMode (Variables|Don'tEdit|GetSkeletal%20Mesh%20Comp) "AnimationBlueprint" true)
        (Class|SkeletalMeshComponent|SetAnimClass (Variables|Don'tEdit|GetSkeletal%20Mesh%20Comp) (Variables|LoadedAssets|GetAnimBP_Class%20-%20Loaded))
        (Animation|Montage|PlayMontage (Variables|Default|GetSkeletal%20Mesh%20Component) "/Game/JumpscarePackX/Animations/AM_RetroTV_Jumpscare_Start_Montage.AM_RetroTV_Jumpscare_Start_Montage"
          (:then
            (CallFunction|LaunchGlass)
            (CallFunction|SpawnSound)
            (CallFunction|PlayCameraShake)
            (bind _returnvalue_2 (Utilities|Time|SetTimerbyEvent (delegate Custom|CustomEvent) 1.0 true))
            (Variables|Don'tEdit|SetLoop%20-%20Timer _returnvalue_2)
            ;;[0 0 0] Physics / Collision - Glass
            (Utilities|Time|SetTimerbyEvent (delegate Custom|CustomEvent_1) 5.0))
          (:OnBlendOut
            ;;[0 0 0] Destroy Mesh
            (Actor|DestroyActor (Variables|Don'tEdit|GetRetro%20TV%20AI)))))
      (:else))
    (else
      (Utilities|Time|SetTimerbyEvent (delegate Custom|CustomEvent_0) 0.1))))

(event EventPrepareJumpscare
  ;[0 0 0] Jumpscare Preload
  (Utilities|FlowControl|DoOnce false
    (:Completed
      (bind _object (Utilities|AsyncLoadAsset (Variables|Settings|Animations|GetMontage))
        (:Completed
          (bind _asanim_montage (Utilities|Casting|CastToAnimMontage _object))
          (Variables|LoadedAssets|SetMontage%20-%20Loaded _asanim_montage)
          (bind _object_2 (Utilities|AsyncLoadAsset (Variables|Settings|GetSkeletal%20Mesh))
            (:Completed
              (bind _asskeletal_mesh (Utilities|Casting|CastToSkeletalMesh _object_2))
              (Variables|LoadedAssets|SetSkeletalMesh%20-%20Loaded _asskeletal_mesh)
              (bind _class (Utilities|AsyncLoadClassAsset (Variables|Settings|GetAnimBP_Class))
                (:Completed
                  (bind _asanim_instance (Utilities|Casting|CastToAnimInstanceClass _class))
                  (Variables|LoadedAssets|SetAnimBP_Class%20-%20Loaded _asanim_instance)
                  (Variables|Don'tEdit|SetReady true))))))))))

(fn ConstructionScript
  (|CallParentFunction))

(fn LaunchGlass
  (bind _arrow (Variables|Default|GetArrow))
  ;[0 0 0] Launch Books
  (if (Variables|Settings|GetOptimized)
    (return)
    (else
      (bind _destroyedscreen (Variables|Default|GetDestroyedScreen)
        (:then
          (LocalVariables|SetGlass%20Array%20L (Components|GetChildrenComponents _destroyedscreen false))
          (for _array_element (LocalVariables|GetGlass%20Array%20L)
            (bind _asstatic_mesh_component (Utilities|Casting|CastToStaticMeshComponent _array_element))
            (Utilities|Array|Add (Variables|Don'tEdit|GetAs%20Static%20Mesh%20Component) _asstatic_mesh_component)
            (Physics|SetSimulatePhysics _asstatic_mesh_component true)
            (Physics|AddForce _asstatic_mesh_component (+ (Transformation|GetWorldLocation _arrow) (* (Math|Vector|GetForwardVector _arrow) (Variables|Settings|GetGlass%20-%20Fall%20Force))) "None" false)
            (Collision|SetCollisionResponsetoChannel _asstatic_mesh_component "ECC_WorldStatic" "ECR_Block")
            (Collision|SetCollisionResponsetoChannel _asstatic_mesh_component "ECC_WorldDynamic" "ECR_Ignore")
            (Collision|SetCollisionEnabled _asstatic_mesh_component "PhysicsOnly"))
          (return))
        (:else
          (return))))))

(fn DestroyGlass
  (params (Glass :type Array%20of%20Scene%20Component%20Object%20References))
  ;[0 0 0] Destroy Glass
  (LocalVariables|SetGlass%20L Glass)
  (for _array_element (LocalVariables|GetGlass%20L)
    (Components|DestroyComponent _array_element))
  (return))