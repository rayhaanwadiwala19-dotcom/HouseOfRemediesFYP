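; BP_ShockLink is a jumpscare actor that shows an animated character in front of the player's camera for a limited time.
; On BeginPlay it attaches to the player character's active camera, using the offset from CharacterData.
; It then async-loads the skeletal mesh, animation and sound in sequence.
; Once loading completes, it plays the sound and looping animation, unhides itself and destroys itself after the configured lifetime.
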(event Custom|CustomEvent
  ;[0 0 0] Begin Play
  ;;[0 0 0] Destroy
  (Actor|DestroyActor))

(event EventBeginPlay
  (bind _character_data (Variables|Default|GetCharacter%20Data))
  (bind (_skeletalmesh _animsequence) (Utilities|Struct|BreakS_Camera_JumpscareData _character_data))
  ;[0 0 0] Begin Play
  ;;[0 0 0] Attach
  (CallFunction|AttachtoPlayerCamera)
  ;;[0 0 0] Load
  (bind _object (Utilities|AsyncLoadAsset _skeletalmesh)
    (:Completed
      (bind _asskeletal_mesh (Utilities|Casting|CastToSkeletalMesh _object))
      (Variables|/Script/Engine.SkeletalMeshComponent|SetSkeletalMeshAsset (Variables|Default|GetSkeletalMesh) _asskeletal_mesh)
      (bind _object_2 (Utilities|AsyncLoadAsset _animsequence)
        (:Completed
          (bind _asanim_sequence (Utilities|Casting|CastToAnimSequence _object_2))
          (Components|Animation|SetAnimation (Variables|Default|GetSkeletalMesh) _asanim_sequence)
          (bind _object_3 (Utilities|AsyncLoadAsset (.Audio (Utilities|Struct|BreakS_Camera_JumpscareData (Variables|Default|GetCharacter%20Data))))
            (:Completed
              (bind _assound_base (Utilities|Casting|CastToSoundBase _object_3)
                (:then
                  (Audio|PlaySound2D _assound_base 1.0 1.0 0.0 0 0))
                (:CastFailed
                  _))
              (Audio|Components|Audio|Play (Variables|Default|GetSkeletalMesh) true)
              (Rendering|SetActorHiddenInGame false)
              (Utilities|Time|SetTimerbyEvent (delegate Custom|CustomEvent) (.Lifetime (Utilities|Struct|BreakS_Camera_JumpscareData (Variables|Default|GetCharacter%20Data)))))))))))

(fn ConstructionScript)

(fn AttachtoPlayerCamera
  (bind _self self)
  (bind _character_data (Variables|Default|GetCharacter%20Data))
  (bind (_skeletalmesh _animsequence _audio _location _rotation) (Utilities|Struct|BreakS_Camera_JumpscareData _character_data))
  ;[0 0 0] Attach To Player Camera
  (for _array_element (Actor|GetComponentsByClass (Game|GetPlayerCharacter 0) "/Script/Engine.CameraComponent")
    (if (Components|Activation|IsActive _array_element)
      (Transformation|AttachComponentToComponent _self _array_element "None" "KeepRelative" "KeepRelative" "KeepRelative" true)
      (Transformation|SetActorRelativeTransform _self (Math|Transform|MakeTransform _location _rotation "1.000000,1.000000,1.000000") false true)
      (return)))
  (return))