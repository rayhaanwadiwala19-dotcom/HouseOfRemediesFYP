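; Interactable rotating painting puzzle piece that solves when its turn count matches PuzzleAnswer.
; Each interaction plays a slide sound and a timeline that pitches the frame by -90 degrees, ignoring input while it moves.
; A match locks the painting, plays an unlock cue and calls the puzzle-completed event.
; Two overlap spheres swap outer and inner prompt icons by player proximity, with sizes and icon placement set in the construction script.
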(event OnComponentBeginOverlap(InnerIconRadius)
  (params (OverlappedComponent :type Primitive%20Component%20Object%20Reference) (OtherActor :type Actor%20Object%20Reference) (OtherComp :type Primitive%20Component%20Object%20Reference) (OtherBodyIndex :type Integer) (bFromSweep :type Boolean) (SweepResult :type Hit%20Result%20Structure%20%28by%20ref%29))
  (if (== OtherActor (Game|GetPlayerCharacter 0))
    (Development|SetHiddeninGame (Variables|Default|GetInnerIcon) false false)
    (Development|SetHiddeninGame (Variables|Default|GetOuterIcon) true false)))

(event OnComponentEndOverlap(InnerIconRadius)
  (params (OverlappedComponent :type Primitive%20Component%20Object%20Reference) (OtherActor :type Actor%20Object%20Reference) (OtherComp :type Primitive%20Component%20Object%20Reference) (OtherBodyIndex :type Integer))
  (if (== (Game|GetPlayerCharacter 0) OtherActor)
    (Development|SetHiddeninGame (Variables|Default|GetInnerIcon) true false)
    (Development|SetHiddeninGame (Variables|Default|GetOuterIcon) false false)))

(event OnComponentBeginOverlap(OuterIconRadius)
  (params (OverlappedComponent :type Primitive%20Component%20Object%20Reference) (OtherActor :type Actor%20Object%20Reference) (OtherComp :type Primitive%20Component%20Object%20Reference) (OtherBodyIndex :type Integer) (bFromSweep :type Boolean) (SweepResult :type Hit%20Result%20Structure%20%28by%20ref%29))
  (if (== OtherActor (Game|GetPlayerCharacter 0))
    (Development|SetHiddeninGame (Variables|Default|GetOuterIcon) false false)))

(event OnComponentEndOverlap(OuterIconRadius)
  (params (OverlappedComponent :type Primitive%20Component%20Object%20Reference) (OtherActor :type Actor%20Object%20Reference) (OtherComp :type Primitive%20Component%20Object%20Reference) (OtherBodyIndex :type Integer))
  (if (== (Game|GetPlayerCharacter 0) OtherActor)
    (Development|SetHiddeninGame (Variables|Default|GetOuterIcon) true false)))

(event Custom|RotatePainting
  (if (not (Variables|Default|GetFrameMoving))
    (Variables|Default|SetFrameMoving true)
    (Audio|PlaySound2D "/Game/InteractionBlueprint/PaintingPuzzle/PaintingPuzzle/Audio/ObjectSlide.ObjectSlide" 1.0 1.0 0.0 0 0)
    (bind _alpha (Timeline|PaintingRotation PlayFromStart)
      (:Update
        (Transformation|SetRelativeRotation (Variables|Default|GetPIctureFrame) (Math|Rotator|MakeRotator 0.0 (Math|Float|Lerp (.pitch (Variables|Default|GetStartingRotationFrame)) (- (.pitch (Variables|Default|GetStartingRotationFrame)) 9e+01) _alpha) 0.0) false false))
      (:Finished
        (Variables|Default|SetStartingRotationFrame (Math|Rotator|MakeRotator 0.0 (Math|Float|Lerp (.pitch (Variables|Default|GetStartingRotationFrame)) (- (.pitch (Variables|Default|GetStartingRotationFrame)) 9e+01) _alpha) 0.0))
        (Variables|Default|SetFrameMoving false)
        (bind _result (Math|Integer|IncrementInt (Variables|Default|GetFramePosition))
          (:%20%20
            (Variables|Default|SetFramePosition _result)
            (if (== (Variables|Default|GetPuzzleAnswer) (Variables|Default|GetFramePosition))
              (Variables|Default|SetFinalised true)
              (Audio|PlaySound2D "/Game/InteractionBlueprint/PaintingPuzzle/PaintingPuzzle/Audio/unlock_Cue.unlock_Cue" 1.0 1.0 0.0 0 0)
              (Default|CallEVDPuzzleCompleted))))))))

(event EventBeginPlay
  (Variables|Default|SetStartingRotationFrame (Variables|/Script/Engine.SceneComponent|GetRelativeRotation (Variables|Default|GetPIctureFrame))))

(event EventInteraction
  (if (not (Variables|Default|GetFinalised))
    (CallFunction|RotatePainting)))

(fn ConstructionScript
  (Utilities|FlowControl|Sequence
    (:then_0
      (|CallParentFunction))
    (:then_1
      (Transformation|SetWorldScale3D (Variables|Default|GetInnerIcon) (Math|Conversions|ToVector(Float) (/ (Variables|Default|GetIconSize) 1e+01)))
      (Transformation|SetRelativeLocation (Variables|Default|GetOuterIcon) (Variables|Default|GetIconLocation) false false))
    (:then_2
      (Components|Sphere|SetSphereRadius (Variables|Default|GetInnerIconRadius) (Variables|Default|GetInnerRadius) true)
      (Components|Sphere|SetSphereRadius (Variables|Default|GetOuterIconRadius) (Variables|Default|GetOuterRadius) true))))