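; Rotating statue puzzle piece for a second-level puzzle, where every statue must face its answer position to complete the puzzle.
; Interaction sets Finalised by comparing the next position to PuzzleAnswer, then a timeline turns the mesh 90 degrees and advances the four-step position.
; Each instance polls all statues on a looping timer, calling the completion event once all are finalised.
; Construction script configures two proximity icons, which overlap spheres show or hide for the player.
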(event OnComponentBeginOverlap(InnerIconRadius)
  (params (OverlappedComponent :type Primitive%20Component%20Object%20Reference) (OtherActor :type Actor%20Object%20Reference) (OtherComp :type Primitive%20Component%20Object%20Reference) (OtherBodyIndex :type Integer) (bFromSweep :type Boolean) (SweepResult :type Hit%20Result%20Structure%20%28by%20ref%29))
  (if (== OtherComp (Game|GetPlayerCharacter 0))
    (Development|SetHiddeninGame (Variables|Default|GetInnerIcon) false false)
    (Development|SetHiddeninGame (Variables|Default|GetOuterIcon) true false)))

(event OnComponentEndOverlap(InnerIconRadius)
  (params (OverlappedComponent :type Primitive%20Component%20Object%20Reference) (OtherActor :type Actor%20Object%20Reference) (OtherComp :type Primitive%20Component%20Object%20Reference) (OtherBodyIndex :type Integer))
  (if (== (Game|GetPlayerCharacter 0) OtherActor)
    (Development|SetHiddeninGame (Variables|Default|GetInnerIcon) true false)
    (Development|SetHiddeninGame (Variables|Default|GetOuterIcon) false false)))

(event OnComponentBeginOverlap(OuterIconRadius)
  (params (OverlappedComponent :type Primitive%20Component%20Object%20Reference) (OtherActor :type Actor%20Object%20Reference) (OtherComp :type Primitive%20Component%20Object%20Reference) (OtherBodyIndex :type Integer) (bFromSweep :type Boolean) (SweepResult :type Hit%20Result%20Structure%20%28by%20ref%29))
  (if (== OtherActor (Game|GetPlayerCharacter 0))
    (Development|SetHiddeninGame (Variables|Default|GetOuterIcon) false false)))

(event OnComponentEndOverlap(OuterIconRadius)
  (params (OverlappedComponent :type Primitive%20Component%20Object%20Reference) (OtherActor :type Actor%20Object%20Reference) (OtherComp :type Primitive%20Component%20Object%20Reference) (OtherBodyIndex :type Integer))
  (if (== (Game|GetPlayerCharacter 0) OtherActor)
    (Development|SetHiddeninGame (Variables|Default|GetOuterIcon) true false)))

(event Custom|RotateCentaur
  (if (not (Variables|Default|GetCentMoving))
    (Variables|Default|SetCentMoving true)
    (Audio|PlaySound2D "/Game/InteractionBlueprint/MonsterDoorStatue/Audio/MonsterMetalMove.MonsterMetalMove" 1.0 1.0 0.0 0 0)
    (bind _alpha (Timeline|CentaurRotation PlayFromStart)
      (:Update
        (Transformation|SetRelativeRotation (Variables|Default|GetSM_Dragon) (Math|Rotator|MakeRotator 0.0 0.0 (Math|Float|Lerp (.yaw (Variables|Default|GetStartingRotationCent)) (- (.yaw (Variables|Default|GetStartingRotationCent)) 9e+01) _alpha)) false false))
      (:Finished
        (Variables|Default|SetStartingRotationCent (Math|Rotator|MakeRotator 0.0 0.0 (Math|Float|Lerp (.yaw (Variables|Default|GetStartingRotationCent)) (- (.yaw (Variables|Default|GetStartingRotationCent)) 9e+01) _alpha)))
        (Variables|Default|SetCentMoving false)
        (bind _result (Math|Integer|IncrementInt (Variables|Default|GetCentPosition))
          (:%20%20
            (bind _output_get (Variables|Default|SetCentPosition _result))
            (if (> _output_get 3)
              (Variables|Default|SetCentPosition 0))))))))

(event Custom|PuzzleCheck
  (Variables|Default|SetPuzzleSolved true)
  (for _array_element (Variables|Default|GetAllCentaurs)
    (if (not (Variables|BP_2ndLevelStatue_Master_Puzzle_C|GetFinalised _array_element))
      (Variables|Default|SetPuzzleSolved false)))
  (if (Variables|Default|GetPuzzleSolved)
    (Utilities|Time|ClearandInvalidateTimerbyHandle (stale EventBeginPlay _returnvalue))
    (Default|CallEVDPuzzleCompleted)))

(event EventBeginPlay
  (Variables|Default|SetStartingRotationCent (Variables|/Script/Engine.SceneComponent|GetRelativeRotation (Variables|Default|GetSM_Dragon)))
  (bind _outactors (Actor|GetAllActorsOfClass "BP_2ndLevelStatue_Master_Puzzle_C"))
  (Variables|Default|SetAllCentaurs _outactors)
  (bind _returnvalue (Utilities|Time|SetTimerbyEvent (delegate Custom|PuzzleCheck) 0.25 true)))

(event EventInteraction
  (if (== (+ (Variables|Default|GetCentPosition) 1) (Variables|Default|GetPuzzleAnswer))
    (Variables|Default|SetFinalised true)
    (CallFunction|RotateCentaur)
    (else
      (Variables|Default|SetFinalised false)
      (CallFunction|RotateCentaur))))

(fn ConstructionScript
  (Utilities|FlowControl|Sequence
    (:then_0
      (|CallParentFunction))
    (:then_1
      (Transformation|SetWorldScale3D (Variables|Default|GetInnerIcon) (Math|Conversions|ToVector(Float) (/ (Variables|Default|GetIconSize) 1e+01)))
      (Transformation|SetRelativeLocation (Variables|Default|GetInnerIcon) (Variables|Default|GetIconLocation) false false))
    (:then_2
      (Components|Sphere|SetSphereRadius (Variables|Default|GetInnerIconRadius) (Variables|Default|GetInnerRadius) true)
      (Components|Sphere|SetSphereRadius (Variables|Default|GetOuterIconRadius) (Variables|Default|GetOuterRadius) true))))