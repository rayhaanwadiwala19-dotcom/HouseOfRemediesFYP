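; Master statue for a rotation puzzle, solved when every statue faces its answer position.
; Interaction sets Finalized by comparing the next position to PuzzleAnswer, then a timeline yaws the statue a quarter turn with a stone-slide sound.
; Each instance polls all statues on a looping timer and fires the puzzle-completed event once all are finalized.
; Overlap spheres swap proximity icons for the player, and Tick prints debug state.
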(event OnComponentBeginOverlap(InnerIconRadius)
  (params (OverlappedComponent :type Primitive%20Component%20Object%20Reference) (OtherActor :type Actor%20Object%20Reference) (OtherComp :type Primitive%20Component%20Object%20Reference) (OtherBodyIndex :type Integer) (bFromSweep :type Boolean) (SweepResult :type Hit%20Result%20Structure%20%28by%20ref%29))
  (if (== OtherActor (Game|GetPlayerCharacter 0))
    (Development|SetHiddeninGame (Variables|Default|GetInnerIcon) false false)
    (Development|SetHiddeninGame (Variables|Default|GetOuterIcon) true false)))

(event OnComponentEndOverlap(InnerIconRadius)
  (params (OverlappedComponent :type Primitive%20Component%20Object%20Reference) (OtherActor :type Actor%20Object%20Reference) (OtherComp :type Primitive%20Component%20Object%20Reference) (OtherBodyIndex :type Integer))
  (if (== (Game|GetPlayerCharacter 0) OtherActor)
    (Development|SetHiddeninGame (Variables|Default|GetInnerIcon) true false)
    (Development|SetHiddeninGame (Variables|Default|GetOuterIcon) false false)))

(event OnComponentBeginOverlap(OuterIconRadius)
  (params (OverlappedComponent :type Primitive%20Component%20Object%20Reference) (OtherActor :type Actor%20Object%20Reference) (OtherComp :type Primitive%20Component%20Object%20Reference) (OtherBodyIndex :type Integer) (bFromSweep :type Boolean) (SweepResult :type Hit%20Result%20Structure%20%28by%20ref%29))
  (if (== OtherActor (Game|GetPlayerCharacter 0))
    (Development|SetHiddeninGame (Variables|Default|GetOuterIcon) false false)))

(event OnComponentEndOverlap(OuterIconRadius)
  (params (OverlappedComponent :type Primitive%20Component%20Object%20Reference) (OtherActor :type Actor%20Object%20Reference) (OtherComp :type Primitive%20Component%20Object%20Reference) (OtherBodyIndex :type Integer))
  (if (== (Game|GetPlayerCharacter 0) OtherActor)
    (Development|SetHiddeninGame (Variables|Default|GetOuterIcon) true false)))

(event Custom|RotatePuzzle
  (if (not (Variables|Default|GetStatueMoving))
    (Variables|Default|SetStatueMoving true)
    (Audio|PlaySound2D "/Game/InteractionBlueprint/PaintingPuzzle/StatuePuzzle/Audio/StoneSlide.StoneSlide" 1.0 1.0 0.0 0 0)
    (bind _rotation (Timeline|StatueRotation PlayFromStart)
      (:Update
        (Transformation|SetRelativeRotation (Variables|Default|GetStatue) (Math|Rotator|MakeRotator 0.0 0.0 (Math|Float|Lerp (.yaw (Variables|Default|GetStatingRotationStatue)) (- (.yaw (Variables|Default|GetStatingRotationStatue)) 9e+01) _rotation)) false false))
      (:Finished
        (Variables|Default|SetStatingRotationStatue (Math|Rotator|MakeRotator 0.0 0.0 (Math|Float|Lerp (.yaw (Variables|Default|GetStatingRotationStatue)) (- (.yaw (Variables|Default|GetStatingRotationStatue)) 9e+01) _rotation)))
        (Variables|Default|SetStatueMoving false)
        (bind _result (Math|Integer|IncrementInt (Variables|Default|GetStatuePosition))
          (:%20%20
            (bind _output_get (Variables|Default|SetStatuePosition _result))
            (if (> _output_get 3)
              (Variables|Default|SetStatuePosition 0))))))))

(event Custom|PuzzleCheck
  (Variables|Default|SetPuzzleSolved true)
  (for _array_element (Variables|Default|GetAllStatues)
    (if (not (Variables|BP_Statue_Master_Puzzle_C|GetFinalized _array_element))
      (Variables|Default|SetPuzzleSolved false)))
  (if (Variables|Default|GetPuzzleSolved)
    (Utilities|Time|ClearandInvalidateTimerbyHandle (stale EventBeginPlay _returnvalue))
    (Default|CallEVDPuzzleCompleted)))

(event EventInteraction
  (if (== (+ (Variables|Default|GetStatuePosition) 1) (Variables|Default|GetPuzzleAnswer))
    (Variables|Default|SetFinalized true)
    (CallFunction|RotatePuzzle)
    (else
      (Variables|Default|SetFinalized false)
      (CallFunction|RotatePuzzle))))

(event EventBeginPlay
  (Variables|Default|SetStatingRotationStatue (Variables|/Script/Engine.SceneComponent|GetRelativeRotation (Variables|Default|GetStatue)))
  (bind _outactors (Actor|GetAllActorsOfClass "BP_Statue_Master_Puzzle_C"))
  (Variables|Default|SetAllStatues _outactors)
  (bind _returnvalue (Utilities|Time|SetTimerbyEvent (delegate Custom|PuzzleCheck) 0.25 true)))

(event EventTick
  (params (DeltaSeconds :type Float%20%28single-precision%29))
  (Development|PrintString (Utilities|String|ToString(Integer) (Variables|Default|GetStatuePosition)) true true "(R=0.000000,G=0.660000,B=1.000000,A=1.000000)" DeltaSeconds)
  (Development|PrintString (Utilities|String|ToString(Boolean) (Variables|Default|GetFinalized)) true true "(R=0.000000,G=0.660000,B=1.000000,A=1.000000)" DeltaSeconds))

(fn ConstructionScript
  (Utilities|FlowControl|Sequence
    (:then_0
      (|CallParentFunction))
    (:then_1
      (Transformation|SetWorldScale3D (Variables|Default|GetInnerIcon) (Math|Conversions|ToVector(Float) (/ (Variables|Default|GetIconSize) 1e+01)))
      (Transformation|SetRelativeLocation (Variables|Default|GetInnerIcon) (Variables|Default|GetIconLocation) false false))
    (:then_2
      (Components|Sphere|SetSphereRadius (Variables|Default|GetInnerIconRadius) (Variables|Default|GetInnerRadius) true)
      (Components|Sphere|SetSphereRadius (Variables|Default|GetOuterIconRadius) (Variables|Default|GetOuterRadius) true))))